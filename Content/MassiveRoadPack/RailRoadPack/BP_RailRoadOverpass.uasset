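; Railroad overpass crossing signal with configurable lights, cross sign and sound.
; Construction script sets the sound and toggles visibility of six lights, their mounts and the secondary sign.
; After a start delay, BeginPlay plays audio and two timelines alternately flash two groups of three lights through dynamic-material EmissivePower.
; With looping on, flashing repeats until Cycles reaches LoopDuration; with it off, audio stops after one cycle.
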(event Custom|Event_PedestrianLoop
  (bind _railcrossinglights_off_interval (Variables|LightAutomation|GetRailCrossingLights%20OFF%20Interval))
  ;[1 1 1] Comment
  (if (Variables|LightAutomation|GetRailCrossingLights%20Loops?)
    (if (not (>= (Variables|LightAutomation|GetCycles) (Variables|LightAutomation|GetLoop%20Duration)))
      (bind _newtrack_0 (Timeline|Timeline_Pedestrian1 PlayFromStart)
        (:Update
          (Rendering|Material|SetScalarParameterValue (Variables|Default|GetPedestrianLightDyn) "EmissivePower" _newtrack_0 :!class /Script/Engine.MaterialInstanceDynamic))
        (:Finished
          (Utilities|FlowControl|Delay _railcrossinglights_off_interval)
          (Components|Timeline|SetPlayRate (Variables|Default|GetTimeline_Pedestrian2) (Variables|LightAutomation|GetLightFlicker%20Speed))
          (bind _newtrack_0_2 (Timeline|Timeline_Pedestrian2 PlayFromStart)
            (:Update
              (Rendering|Material|SetScalarParameterValue (Variables|Default|GetPedestrianLightDyn2) "EmissivePower" _newtrack_0_2 :!class /Script/Engine.MaterialInstanceDynamic))
            (:Finished
              (Utilities|FlowControl|Delay _railcrossinglights_off_interval)
              (Variables|LightAutomation|SetCycles (+ (Variables|LightAutomation|GetCycles) 1))
              (CallFunction|EventPedestrianLoop))))))
    (else
      (Audio|Components|Audio|Stop (Variables|Default|GetAudio)))))

(event EventBeginPlay
  (bind _light1 (Variables|Default|GetLight1))
  (bind _light3 (Variables|Default|GetLight3))
  (bind _audio (Variables|Default|GetAudio))
  (bind _light4 (Variables|Default|GetLight4))
  (bind _lightflicker_speed (Variables|LightAutomation|GetLightFlicker%20Speed))
  (bind _light2 (Variables|Default|GetLight2))
  (bind _railcrossinglights_off_interval (Variables|LightAutomation|GetRailCrossingLights%20OFF%20Interval))
  (bind _light6 (Variables|Default|GetLight6))
  (bind _light5 (Variables|Default|GetLight5))
  ;[1 1 1] Comment
  (Utilities|FlowControl|Sequence
    (:then_0
      (if (Variables|LightAutomation|GetRailCrossingLights%20Operating?)
        (Utilities|FlowControl|Sequence
          (:then_0
            (Utilities|FlowControl|Sequence
              (:then_0
                (bind _returnvalue (Rendering|Material|CreateDynamicMaterialInstance _light1 0 (Rendering|Material|GetMaterial _light1 0) :!class /Script/Engine.PrimitiveComponent))
                (Variables|Default|SetPedestrianLightDyn _returnvalue))
              (:then_1
                (bind _returnvalue_2 (Rendering|Material|CreateDynamicMaterialInstance _light3 0 (Rendering|Material|GetMaterial _light3 0) :!class /Script/Engine.PrimitiveComponent))
                (Variables|Default|SetPedestrianLightDyn3 _returnvalue_2))
              (:then_2
                (bind _returnvalue_3 (Rendering|Material|CreateDynamicMaterialInstance _light2 0 (Rendering|Material|GetMaterial _light2 0) :!class /Script/Engine.PrimitiveComponent))
                (Variables|Default|SetPedestrianLightDyn2 _returnvalue_3))
              (:then_3
                (bind _returnvalue_4 (Rendering|Material|CreateDynamicMaterialInstance _light4 0 (Rendering|Material|GetMaterial _light4 0) :!class /Script/Engine.PrimitiveComponent))
                (Variables|Default|SetPedestrianLightDyn4 _returnvalue_4))
              (:then_4
                (bind _returnvalue_5 (Rendering|Material|CreateDynamicMaterialInstance _light5 0 (Rendering|Material|GetMaterial _light5 0) :!class /Script/Engine.PrimitiveComponent))
                (Variables|Default|SetPedestrianLightDyn5 _returnvalue_5))
              (:then_5
                (bind _returnvalue_6 (Rendering|Material|CreateDynamicMaterialInstance _light6 0 (Rendering|Material|GetMaterial _light6 0) :!class /Script/Engine.PrimitiveComponent))
                (Variables|Default|SetPedestrianLightDyn6 _returnvalue_6))))
          (:then_1
            (Utilities|FlowControl|Delay (Variables|LightAutomation|GetRailCrossingLights%20StartDelay))
            (Utilities|IsValid _audio
              (:Is%20Valid
                (Audio|Components|Audio|Play _audio 0.0)
                (Components|Timeline|SetPlayRate (Variables|Default|GetTimeline_Pedestrian1) _lightflicker_speed)
                (bind _newtrack_0 (Timeline|Timeline_Pedestrian1 PlayFromStart)
                  (:Update
                    (Rendering|Material|SetScalarParameterValue (Variables|Default|GetPedestrianLightDyn) "EmissivePower" _newtrack_0 :!class /Script/Engine.MaterialInstanceDynamic))
                  (:Finished
                    (Utilities|FlowControl|Delay _railcrossinglights_off_interval)
                    (Components|Timeline|SetPlayRate (Variables|Default|GetTimeline_Pedestrian2) _lightflicker_speed)
                    (bind _newtrack_0_2 (Timeline|Timeline_Pedestrian2 PlayFromStart)
                      (:Update
                        (Rendering|Material|SetScalarParameterValue (Variables|Default|GetPedestrianLightDyn2) "EmissivePower" _newtrack_0_2 :!class /Script/Engine.MaterialInstanceDynamic))
                      (:Finished
                        (Utilities|FlowControl|Delay _railcrossinglights_off_interval)
                        (Variables|LightAutomation|SetCycles (+ (Variables|LightAutomation|GetCycles) 1))
                        (CallFunction|EventPedestrianLoop)))))))))))))

(fn ConstructionScript
  (Utilities|FlowControl|Sequence
    (:then_0
      ;[1 1 1] Asset Parts Selection
      (Audio|Components|Audio|SetSound (Variables|Default|GetAudio) (Variables|LightAutomation|GetSelect%20Sound)))
    (:then_1
      (Rendering|SetVisibility (Variables|Default|GetLight1) (Variables|Default|GetLight1?) false))
    (:then_2
      (Rendering|SetVisibility (Variables|Default|GetLight2) (Variables|Default|GetLight2?) false))
    (:then_3
      (Rendering|SetVisibility (Variables|Default|GetLight3) (Variables|Default|GetLight3?) false))
    (:then_4
      (Rendering|SetVisibility (Variables|Default|GetLight4) (Variables|Default|GetLight4?) false))
    (:then_5
      (if (and (not (Variables|Default|GetLight1?)) (not (Variables|Default|GetLight2?)))
        (Rendering|SetVisibility (Variables|Default|GetMainLightConnector) false false)))
    (:then_6
      (if (and (not (Variables|Default|GetLight3?)) (not (Variables|Default|GetLight4?)))
        (Rendering|SetVisibility (Variables|Default|GetOverpassLights_LightGroup1) false false)))
    (:then_7
      (if (and (not (Variables|Default|GetLight5?)) (not (Variables|Default|GetLight6?)))
        (Rendering|SetVisibility (Variables|Default|GetOverpassLights_LightGroup2) false false)))
    (:then_8
      (Rendering|SetVisibility (Variables|Default|GetLight5) (Variables|Default|GetLight5?) false))
    (:then_9
      (Rendering|SetVisibility (Variables|Default|GetLight6) (Variables|Default|GetLight6?) false))
    (:then_10
      (Rendering|SetVisibility (Variables|Default|GetCrossSignMount2) (Variables|Default|GetSecondaryCrossSign?) false))))