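; Railroad crossing signal actor with flashing lights, warning audio and an optional rotating blockade arm.
; The construction script sets the sound and shows or hides lights, arms and blockade parts from the chosen options.
; After a start delay, if enabled, BeginPlay lowers the blockade and alternates two timelines driving emissive power on dynamic materials.
; A cycle counter ends the flashing, stops audio, raises the blockade and optionally restarts after an interval.
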(event Custom|RailRoadBlock_LOOP
  (bind _audio (Variables|Default|GetAudio))
  (bind _off_interval (Variables|LightAutomation|GetOFF%20Interval))
  (bind _audio_2 (Variables|Default|GetAudio))
  (bind _lightflicker_speed (Variables|Lights|GetLightFlicker%20Speed))
  (bind _lightsflickeroff_interval (Variables|Lights|GetLightsFlickerOFF%20Interval))
  ;[1 0.5098 0.4999] Rotates blockade
  (Variables|LightAutomation|SetCycles 0)
  (if (Variables|LightAutomation|GetRailRoadBlockade?)
    (Utilities|FlowControl|Sequence
      (:then_0
        (bind _rotate (Timeline|Timeline_blockadeDown PlayFromStart)
          (:Update
            (Transformation|SetRelativeRotation (Variables|Default|GetBlockade) (Math|Rotator|MakeRotator 0.0 _rotate 0.0) false false))))
      (:then_1
        ;[1 0.4755 0] Light Loop Operation
        (if (>= (Variables|LightAutomation|GetCycles) (Variables|LightAutomation|GetLoop%20Duration))
          ;[1 0.5098 0.4999] Turns Blockage OFF (Up position)
          (if (Variables|LightAutomation|GetRailRoadBlockade?)
            (Audio|Components|Audio|Stop _audio_2)
            (CallFunction|EventSDFXReset)
            (bind _rotate_2 (Timeline|Timeline_BlockadeUP PlayFromStart)
              (:Update
                (Transformation|SetRelativeRotation (Variables|Default|GetBlockade) (Math|Rotator|MakeRotator 0.0 _rotate_2 0.0) false false))
              (:Finished
                ;[1 1 1] STOP + LOOPING OPERATIONS
                (if (Variables|LightAutomation|GetRailRoadBlock_Loop?)
                  (Utilities|FlowControl|Delay _off_interval)
                  (CallFunction|RailRoadBlockLOOP))))
            (else
              (Audio|Components|Audio|Stop _audio_2)
              (CallFunction|EventSDFXReset)
              (if (Variables|LightAutomation|GetRailCrossingLights%20Loops?)
                (Utilities|FlowControl|Delay _off_interval)
                (Variables|LightAutomation|SetCycles 0)
                (CallFunction|EventPedestrianLoop))))
          (else
            (Utilities|IsValid _audio
              (:Is%20Valid
                (Utilities|FlowControl|Sequence
                  (:then_0
                    (Utilities|FlowControl|DoOnce false
                      (:Completed
                        (Audio|Components|Audio|Play _audio 0.0))))
                  (:then_1
                    (Components|Timeline|SetPlayRate (Variables|Default|GetTimeline_Pedestrian1) _lightflicker_speed :!label _label)
                    (bind _newtrack_0 (Timeline|Timeline_Pedestrian1 PlayFromStart)
                      (:Update
                        (Rendering|Material|SetScalarParameterValue (Variables|Default|GetPedestrianLightDyn) "EmissivePower" _newtrack_0 :!class /Script/Engine.MaterialInstanceDynamic))
                      (:Finished
                        (Utilities|FlowControl|Delay _lightsflickeroff_interval)
                        (Components|Timeline|SetPlayRate (Variables|Default|GetTimeline_Pedestrian2) _lightflicker_speed)
                        (bind _newtrack_0_2 (Timeline|Timeline_Pedestrian2 PlayFromStart)
                          (:Update
                            (Rendering|Material|SetScalarParameterValue (Variables|Default|GetPedestrianLightDyn2) "EmissivePower" _newtrack_0_2 :!class /Script/Engine.MaterialInstanceDynamic))
                          (:Finished
                            (Utilities|FlowControl|Delay _lightsflickeroff_interval)
                            (Variables|LightAutomation|SetCycles (+ (Variables|LightAutomation|GetCycles) 1))
                            (CallFunction|EventPedestrianLoop))))))))
              (:Is%20Not%20Valid
                (goto _label)))))))))

(event Custom|Event_PedestrianLoop
  (bind _audio (Variables|Default|GetAudio))
  (bind _off_interval (Variables|LightAutomation|GetOFF%20Interval))
  (bind _audio_2 (Variables|Default|GetAudio))
  (bind _lightflicker_speed (Variables|Lights|GetLightFlicker%20Speed))
  (bind _lightsflickeroff_interval (Variables|Lights|GetLightsFlickerOFF%20Interval))
  ;[1 0.4755 0] Light Loop Operation
  (if (>= (Variables|LightAutomation|GetCycles) (Variables|LightAutomation|GetLoop%20Duration))
    ;[1 0.5098 0.4999] Turns Blockage OFF (Up position)
    (if (Variables|LightAutomation|GetRailRoadBlockade?)
      (Audio|Components|Audio|Stop _audio_2)
      (CallFunction|EventSDFXReset)
      (bind _rotate (Timeline|Timeline_BlockadeUP PlayFromStart)
        (:Update
          (Transformation|SetRelativeRotation (Variables|Default|GetBlockade) (Math|Rotator|MakeRotator 0.0 _rotate 0.0) false false))
        (:Finished
          ;[1 1 1] STOP + LOOPING OPERATIONS
          (if (Variables|LightAutomation|GetRailRoadBlock_Loop?)
            (Utilities|FlowControl|Delay _off_interval)
            (CallFunction|RailRoadBlockLOOP))))
      (else
        (Audio|Components|Audio|Stop _audio_2)
        (CallFunction|EventSDFXReset)
        (if (Variables|LightAutomation|GetRailCrossingLights%20Loops?)
          (Utilities|FlowControl|Delay _off_interval)
          (Variables|LightAutomation|SetCycles 0)
          (CallFunction|EventPedestrianLoop))))
    (else
      (Utilities|IsValid _audio
        (:Is%20Valid
          (Utilities|FlowControl|Sequence
            (:then_0
              (Utilities|FlowControl|DoOnce false
                (:Completed
                  (Audio|Components|Audio|Play _audio 0.0))))
            (:then_1
              (Components|Timeline|SetPlayRate (Variables|Default|GetTimeline_Pedestrian1) _lightflicker_speed :!label _label)
              (bind _newtrack_0 (Timeline|Timeline_Pedestrian1 PlayFromStart)
                (:Update
                  (Rendering|Material|SetScalarParameterValue (Variables|Default|GetPedestrianLightDyn) "EmissivePower" _newtrack_0 :!class /Script/Engine.MaterialInstanceDynamic))
                (:Finished
                  (Utilities|FlowControl|Delay _lightsflickeroff_interval)
                  (Components|Timeline|SetPlayRate (Variables|Default|GetTimeline_Pedestrian2) _lightflicker_speed)
                  (bind _newtrack_0_2 (Timeline|Timeline_Pedestrian2 PlayFromStart)
                    (:Update
                      (Rendering|Material|SetScalarParameterValue (Variables|Default|GetPedestrianLightDyn2) "EmissivePower" _newtrack_0_2 :!class /Script/Engine.MaterialInstanceDynamic))
                    (:Finished
                      (Utilities|FlowControl|Delay _lightsflickeroff_interval)
                      (Variables|LightAutomation|SetCycles (+ (Variables|LightAutomation|GetCycles) 1))
                      (CallFunction|EventPedestrianLoop))))))))
        (:Is%20Not%20Valid
          (goto _label))))))

(event Custom|Event_SDFXReset
  ;[1 0.4755 0] Light Loop Operation
  (Utilities|FlowControl|DoOnce false) ; enters at Reset
)

(event EventBeginPlay
  (bind _light1 (Variables|Default|GetLight1))
  (bind _light3 (Variables|Default|GetLight3))
  (bind _audio (Variables|Default|GetAudio))
  (bind _off_interval (Variables|LightAutomation|GetOFF%20Interval))
  (bind _audio_2 (Variables|Default|GetAudio))
  (bind _light4 (Variables|Default|GetLight4))
  (bind _lightflicker_speed (Variables|Lights|GetLightFlicker%20Speed))
  (bind _blockadelights1 (Variables|Default|GetBlockadeLights1))
  (bind _blockadelights2 (Variables|Default|GetBlockadeLights2))
  (bind _blockadelights (Variables|Default|GetBlockadeLights))
  (bind _light2 (Variables|Default|GetLight2))
  (bind _lightsflickeroff_interval (Variables|Lights|GetLightsFlickerOFF%20Interval))
  ;[1 1 1] Begin Play Automation
  (Utilities|FlowControl|Delay (Variables|LightAutomation|GetON%20Delay))
  (if (Variables|LightAutomation|GetRailCrossingLights%20ON?)
    (Utilities|FlowControl|Sequence
      (:then_0
        ;[1 1 1] Create Dynamice Materials to animate lights
        (Utilities|FlowControl|Sequence
          (:then_0
            (bind _returnvalue (Rendering|Material|CreateDynamicMaterialInstance _blockadelights 0 (Rendering|Material|GetMaterial _blockadelights 0) :!class /Script/Engine.PrimitiveComponent))
            (Variables|Default|SetBlockadeLight0DYN _returnvalue))
          (:then_1
            (bind _returnvalue_2 (Rendering|Material|CreateDynamicMaterialInstance _blockadelights1 0 (Rendering|Material|GetMaterial _blockadelights1 0) :!class /Script/Engine.PrimitiveComponent))
            (Variables|Default|SetBlockadeLight1DYN _returnvalue_2))
          (:then_2
            (bind _returnvalue_3 (Rendering|Material|CreateDynamicMaterialInstance _blockadelights2 0 (Rendering|Material|GetMaterial _blockadelights2 0) :!class /Script/Engine.PrimitiveComponent))
            (Variables|Default|SetBlockadeLight2DYN _returnvalue_3))))
      (:then_1
        (Utilities|FlowControl|Sequence
          (:then_0
            (bind _returnvalue_4 (Rendering|Material|CreateDynamicMaterialInstance _light1 0 (Rendering|Material|GetMaterial _light1 0) :!class /Script/Engine.PrimitiveComponent))
            (Variables|Default|SetPedestrianLightDyn _returnvalue_4))
          (:then_1
            (bind _returnvalue_5 (Rendering|Material|CreateDynamicMaterialInstance _light3 0 (Rendering|Material|GetMaterial _light3 0) :!class /Script/Engine.PrimitiveComponent))
            (Variables|Default|SetPedestrianLightDyn3 _returnvalue_5))
          (:then_2
            (bind _returnvalue_6 (Rendering|Material|CreateDynamicMaterialInstance _light2 0 (Rendering|Material|GetMaterial _light2 0) :!class /Script/Engine.PrimitiveComponent))
            (Variables|Default|SetPedestrianLightDyn2 _returnvalue_6))
          (:then_3
            (bind _returnvalue_7 (Rendering|Material|CreateDynamicMaterialInstance _light4 0 (Rendering|Material|GetMaterial _light4 0) :!class /Script/Engine.PrimitiveComponent))
            (Variables|Default|SetPedestrianLightDyn4 _returnvalue_7))))
      (:then_2
        ;[1 0.5098 0.4999] Rotates blockade
        (if (Variables|LightAutomation|GetRailRoadBlockade?)
          (Utilities|FlowControl|Sequence
            (:then_0
              (bind _rotate (Timeline|Timeline_blockadeDown PlayFromStart)
                (:Update
                  (Transformation|SetRelativeRotation (Variables|Default|GetBlockade) (Math|Rotator|MakeRotator 0.0 _rotate 0.0) false false))))
            (:then_1
              ;[1 0.4755 0] Light Loop Operation
              (if (>= (Variables|LightAutomation|GetCycles) (Variables|LightAutomation|GetLoop%20Duration)) :!label _label
                ;[1 0.5098 0.4999] Turns Blockage OFF (Up position)
                (if (Variables|LightAutomation|GetRailRoadBlockade?)
                  (Audio|Components|Audio|Stop _audio_2)
                  (CallFunction|EventSDFXReset)
                  (bind _rotate_2 (Timeline|Timeline_BlockadeUP PlayFromStart)
                    (:Update
                      (Transformation|SetRelativeRotation (Variables|Default|GetBlockade) (Math|Rotator|MakeRotator 0.0 _rotate_2 0.0) false false))
                    (:Finished
                      ;[1 1 1] STOP + LOOPING OPERATIONS
                      (if (Variables|LightAutomation|GetRailRoadBlock_Loop?)
                        (Utilities|FlowControl|Delay _off_interval)
                        (CallFunction|RailRoadBlockLOOP))))
                  (else
                    (Audio|Components|Audio|Stop _audio_2)
                    (CallFunction|EventSDFXReset)
                    (if (Variables|LightAutomation|GetRailCrossingLights%20Loops?)
                      (Utilities|FlowControl|Delay _off_interval)
                      (Variables|LightAutomation|SetCycles 0)
                      (CallFunction|EventPedestrianLoop))))
                (else
                  (Utilities|IsValid _audio
                    (:Is%20Valid
                      (Utilities|FlowControl|Sequence
                        (:then_0
                          (Utilities|FlowControl|DoOnce false
                            (:Completed
                              (Audio|Components|Audio|Play _audio 0.0))))
                        (:then_1
                          (Components|Timeline|SetPlayRate (Variables|Default|GetTimeline_Pedestrian1) _lightflicker_speed :!label _label_2)
                          (bind _newtrack_0 (Timeline|Timeline_Pedestrian1 PlayFromStart)
                            (:Update
                              (Rendering|Material|SetScalarParameterValue (Variables|Default|GetPedestrianLightDyn) "EmissivePower" _newtrack_0 :!class /Script/Engine.MaterialInstanceDynamic))
                            (:Finished
                              (Utilities|FlowControl|Delay _lightsflickeroff_interval)
                              (Components|Timeline|SetPlayRate (Variables|Default|GetTimeline_Pedestrian2) _lightflicker_speed)
                              (bind _newtrack_0_2 (Timeline|Timeline_Pedestrian2 PlayFromStart)
                                (:Update
                                  (Rendering|Material|SetScalarParameterValue (Variables|Default|GetPedestrianLightDyn2) "EmissivePower" _newtrack_0_2 :!class /Script/Engine.MaterialInstanceDynamic))
                                (:Finished
                                  (Utilities|FlowControl|Delay _lightsflickeroff_interval)
                                  (Variables|LightAutomation|SetCycles (+ (Variables|LightAutomation|GetCycles) 1))
                                  (CallFunction|EventPedestrianLoop))))))))
                    (:Is%20Not%20Valid
                      (goto _label_2)))))))))
      (:then_3
        (goto _label)))))

(fn ConstructionScript
  (Utilities|FlowControl|Sequence
    (:then_0
      ;[1 1 1] Asset Parts Selection
      (Audio|Components|Audio|SetSound (Variables|Default|GetAudio) (Variables|LightAutomation|GetSelect%20Sound)))
    (:then_1
      (Rendering|SetVisibility (Variables|Default|GetLight1) (Variables|Lights|GetLight1?) false))
    (:then_2
      (Rendering|SetVisibility (Variables|Default|GetArmShort2) (Variables|Lights|GetLight2?) false))
    (:then_3
      (Rendering|SetVisibility (Variables|Default|GetArmLong1) (Variables|Lights|GetLight3?) false))
    (:then_4
      (Rendering|SetVisibility (Variables|Default|GetLight4) (Variables|Lights|GetLight4?) false))
    (:then_5
      (if (Math|Boolean|ANDBoolean (not (Variables|Lights|GetLight1?)) (not (Variables|Lights|GetLight2?)) (not (Variables|Lights|GetLight3?)) (not (Variables|Lights|GetLight4?)))
        (Rendering|SetVisibility (Variables|Default|GetMainLightConnector) false false)))
    (:then_6
      (if (Variables|LightAutomation|GetRailRoadBlockade?)
        (Utilities|FlowControl|Sequence
          (:then_0
            (Rendering|SetVisibility (Variables|Default|GetRailCrossBlockade_Blockade) true false))
          (:then_1
            (Rendering|SetVisibility (Variables|Default|GetLight3) false false)))))))