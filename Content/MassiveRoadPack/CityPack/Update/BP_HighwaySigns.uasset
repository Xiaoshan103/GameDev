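; Configurable highway sign prop that builds either a pole-mounted main sign, an overpass gantry, or both from exposed options in the Construction Script.
; Flags toggle visibility and collision of pre-placed meshes for single, dual or no poles, two-sided, full-span or platform gantries, and optional end-pole removal.
; Per-sign functions fill three text and number rows from arrays and reveal optional decals, with custom materials on gantry signs; platform mode suppresses opposite-side signs.
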(fn ConstructionScript
  (bind _mainsign (Variables|Default|GetMAINSIGN))
  (bind _overpass_1duo (Variables|Default|GetOVERPASS%201DUO))
  (bind _overpass_2 (Variables|Default|GetOVERPASS%202))
  (bind _overpass_2_2 (Variables|Default|GetOVERPASS%202))
  (bind _overpass_1 (Variables|Default|GetOVERPASS%201))
  (bind _ibeam1 (Variables|Default|GetIBEAM1))
  (bind _ibeam1_2 (Variables|Default|GetIBEAM1))
  (bind _full_overpass_ (Variables|OVERPASSSIGN|GetFULL%20Overpass?))
  (bind _ibeam1_3 (Variables|Default|GetIBEAM1))
  (Utilities|FlowControl|Sequence
    (:then_1
      ;[1 1 1] Main Sign Settings
      (if (Variables|MAINSIGN|GetMAIN%20SIGN?)
        (if (Variables|MAINSIGN|GetDual%20Poles?)
          (Rendering|SetVisibility (Variables|Default|GetIBEAM2) true false)
          (Collision|SetCollisionEnabled _ibeam1_3 "QueryAndPhysics")
          (Transformation|AddRelativeLocation _ibeam1_3 (Math|Vector|MakeVector 1e+02 0.0 0.0) false false)
          (else
            (Rendering|SetVisibility _ibeam1 true false)
            (Collision|SetCollisionEnabled _ibeam1 "QueryAndPhysics")
            (Transformation|AddRelativeLocation _ibeam1 (Math|Vector|MakeVector 0.0 0.0 0.0) false false)))
        (Rendering|SetVisibility _mainsign true false)
        (Collision|SetCollisionEnabled _mainsign "QueryAndPhysics")
        (if (Variables|MAINSIGN|GetNo%20Pole?)
          (Rendering|SetVisibility _ibeam1_2 false false)
          (Collision|SetCollisionEnabled _ibeam1_2 "NoCollision"))
        (|SetSignDetailsMain)
        (else
          (Rendering|SetVisibility _mainsign false false))))
    (:then_2
      ;[1 1 1] OverPass Settings
      (if (Variables|OVERPASSSIGN|GetOVERPASS?)
        (Utilities|FlowControl|Sequence
          (:then_0
            (Rendering|SetVisibility _overpass_1 true false)
            (if (Variables|OVERPASSSIGN|GetDUO%20SIDED?)
              (Rendering|SetVisibility _overpass_1duo true false)
              (Collision|SetCollisionEnabled (Variables|Default|GetOVERPASS%20POLES%201DUO) "QueryAndPhysics")
              (Components|StaticMesh|SetStaticMesh _overpass_1 "/Game/MassiveRoadPack/CityPack/Meshes/Update/SM_OverPassStructureA.SM_OverPassStructureA")
              (if _full_overpass_
                (Rendering|SetVisibility _overpass_2_2 true false)
                (Components|StaticMesh|SetStaticMesh _overpass_2_2 "/Game/MassiveRoadPack/CityPack/Meshes/Update/SM_OverPassStructureA.SM_OverPassStructureA")
                (Collision|SetCollisionEnabled (Variables|Default|GetOVERPASS%202DUO) "QueryAndPhysics")
                (if (Variables|OVERPASSSIGN|GetRemove%20Poles%20At%20End?) :!label _label
                  (Rendering|SetVisibility (Variables|Default|GetOVERPASS%20POLES%202) false false)
                  (Collision|SetCollisionEnabled (Variables|Default|GetOVERPASS%20POLES%202DUO) "NoCollision")))
              (elif (Variables|OVERPASSSIGN|GetPlatform?)
                (Utilities|FlowControl|Sequence
                  (:then_0
                    (Rendering|SetVisibility _overpass_1duo false false)
                    (Components|StaticMesh|SetStaticMesh (Variables|Default|GetOVERPASS%201) "/Game/MassiveRoadPack/CityPack/Meshes/Update/SM_OverPassStructureA.SM_OverPassStructureA")
                    (if _full_overpass_
                      (Rendering|SetVisibility _overpass_2 true false)
                      (Components|StaticMesh|SetStaticMesh _overpass_2 "/Game/MassiveRoadPack/CityPack/Meshes/Update/SM_OverPassStructureA.SM_OverPassStructureA")
                      (Collision|SetCollisionEnabled _overpass_2 "QueryAndPhysics" :!label _label_2)
                      (goto _label)))
                  (:then_1
                    (Variables|Default|SetOppositeSignsOFF true)))
                (else
                  (Rendering|SetVisibility _overpass_1duo false false)
                  (Transformation|AddRelativeLocation (Variables|Default|GetSIGN%20F) "0.000000,60.000000, 0" false false)
                  (if _full_overpass_
                    (Rendering|SetVisibility _overpass_2 true false)
                    (goto _label_2))))))
          (:then_1
            ;[1 1 1] Set Signs
            (Utilities|FlowControl|Sequence
              (:then_0
                (|SetSignDetailsA))
              (:then_1
                (|SetSignDetailsB))
              (:then_2
                (|SetSignDetailsC))
              (:then_3
                (|SetSignDetailsD))
              (:then_4
                (if (Variables|SIGNOPPOSITEA|GetSign%20Opposite%20A?)
                  (if (Variables|Default|GetOppositeSignsOFF)
                    (Rendering|SetVisibility (Variables|Default|GetSIGN%20E) false false)
                    (else
                      (|SetSignDetailsE)))))
              (:then_5
                (if (Variables|SIGNOPPOSITEB|GetSign%20Opposite%20B?)
                  (if (Variables|Default|GetOppositeSignsOFF)
                    (Rendering|SetVisibility (Variables|Default|GetSIGN%20F) false false)
                    (else
                      (|SetSignDetailsF)))))))
          (:then_2
            (Collision|SetCollisionEnabled (Variables|Default|GetOVERPASS%20POLES%201) "QueryAndPhysics")))))))