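; Spline-driven power line tool that builds a row of poles joined by cables in the construction script.
; It spawns a pole child actor at each spline point, rotates it to the spline and can drop it onto a line-traced surface.
; A second pass attaches each pole's two cables to the next pole's connectors, sets length from distance plus random slack and zeroes the last pole's cables.
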(event EventBeginPlay)

(event Collision|EventActorBeginOverlap
  (params (OtherActor :type Actor%20Object%20Reference)))

(event EventTick
  (params (DeltaSeconds :type Float%20%28single-precision%29)))

(fn ConstructionScript
  (bind _spline (Variables|Default|GetSpline))
  (bind _powerpole_array (Variables|Default|GetPowerPole%20Array))
  (bind _random_powerline_length (Variables|Default|GetRandom%20PowerLine%20Length))
  ;[1 1 1] Spawns Polerline BP along Spline Points
  (bind _output_get (Variables|Default|SetNumberOfSplinePoints (- (Spline|GetNumberOfSplinePoints (Variables|Default|GetSpline)) 1)))
  (for _index (range 0 _output_get)
    (Variables|Default|SetIndex%20Loop _index)
    ;[1 1 1] Sets Location of Powepoles to Surface Dectected below
    (bind _outhit (Collision|LineTraceByChannel (Math|Vector|MakeVector (.x (Spline|GetLocationatSplinePoint (Variables|Default|GetSpline) (Variables|Default|GetIndex%20Loop) "World")) (.y (Spline|GetLocationatSplinePoint (Variables|Default|GetSpline) (Variables|Default|GetIndex%20Loop) "World")) (.z (Spline|GetLocationatSplinePoint (Variables|Default|GetSpline) (Variables|Default|GetIndex%20Loop) "World"))) (Math|Vector|MakeVector (.x (Spline|GetLocationatSplinePoint (Variables|Default|GetSpline) (Variables|Default|GetIndex%20Loop) "World")) (.y (Spline|GetLocationatSplinePoint (Variables|Default|GetSpline) (Variables|Default|GetIndex%20Loop) "World")) (Variables|Default|GetSurfaceTraceLength)) "TraceTypeQuery1" false 0 "ForOneFrame"))
    (bind _returnvalue (AddComponent|AddChildActorComponent false (Math|Conversions|ToTransform(Vector) (Spline|GetLocationatSplinePoint _spline (Variables|Default|GetIndex%20Loop) "Local"))))
    (if (Variables|Default|GetAlign%20to%20Surface?)
      (Transformation|SetWorldLocation _returnvalue (.Location (Collision|BreakHitResult _outhit)) false false))
    (ChildActorComponent|SetChildActorClass _returnvalue (Variables|Default|GetPowerLinePole))
    (bind _asbp_power_poles_spline (Utilities|Casting|CastToBP_PowerPolesSpline (Variables|/Script/Engine.ChildActorComponent|GetChildActor _returnvalue)))
    (Utilities|Array|Add (Variables|Default|GetPowerPole%20Array) _asbp_power_poles_spline)
    (Transformation|SetRelativeRotation _returnvalue (Spline|GetRotationatSplinePoint _spline (Variables|Default|GetIndex%20Loop) "Local") false false))
  ;[1 1 1] Attaches Cables to Connectors on next pole in spline point index
  (for _index_2 (range 0 (Variables|Default|GetNumberOfSplinePoints))
    (Variables|Default|SetIndex%20Loop2 _index_2)
    (Utilities|FlowControl|Sequence
      (:then_0
        (Transformation|AttachComponentToComponent (Variables|/Game/MassiveRoadPack/CityPack/Update/BP_PowerPolesSpline.BP_PowerPolesSpline_C|GetCable1 (Utilities|Array|Get(acopy) _powerpole_array (Variables|Default|GetIndex%20Loop2))) (Variables|/Game/MassiveRoadPack/CityPack/Update/BP_PowerPolesSpline.BP_PowerPolesSpline_C|GetConnect1 (Utilities|Array|Get(acopy) _powerpole_array (+ (Variables|Default|GetIndex%20Loop2) 1))) "None" "SnapToTarget" "SnapToTarget" "KeepWorld" true)
        (Variables|/Script/CableComponent.CableComponent|SetCableLength (Variables|/Game/MassiveRoadPack/CityPack/Update/BP_PowerPolesSpline.BP_PowerPolesSpline_C|GetCable1 (Utilities|Array|Get(acopy) _powerpole_array (Variables|Default|GetIndex%20Loop2))) (+ (Math|Vector|VectorLength (- (Transformation|GetWorldLocation (Variables|/Game/MassiveRoadPack/CityPack/Update/BP_PowerPolesSpline.BP_PowerPolesSpline_C|GetConnect1 (Utilities|Array|Get(acopy) _powerpole_array (Variables|Default|GetIndex%20Loop2)))) (Transformation|GetWorldLocation (Variables|/Game/MassiveRoadPack/CityPack/Update/BP_PowerPolesSpline.BP_PowerPolesSpline_C|GetConnect1 (Utilities|Array|Get(acopy) _powerpole_array (+ (Variables|Default|GetIndex%20Loop2) 1)))))) (Math|Random|RandomFloatinRange 0.0 _random_powerline_length)))
        (Variables|/Script/CableComponent.CableComponent|SetCableLength (Variables|/Game/MassiveRoadPack/CityPack/Update/BP_PowerPolesSpline.BP_PowerPolesSpline_C|GetCable1 (Utilities|Array|Get(acopy) (Variables|Default|GetPowerPole%20Array) (Variables|Default|GetNumberOfSplinePoints))) 0.0))
      (:then_1
        (Transformation|AttachComponentToComponent (Variables|/Game/MassiveRoadPack/CityPack/Update/BP_PowerPolesSpline.BP_PowerPolesSpline_C|GetCable2 (Utilities|Array|Get(acopy) _powerpole_array (Variables|Default|GetIndex%20Loop2))) (Variables|/Game/MassiveRoadPack/CityPack/Update/BP_PowerPolesSpline.BP_PowerPolesSpline_C|GetConnect2 (Utilities|Array|Get(acopy) _powerpole_array (+ (Variables|Default|GetIndex%20Loop2) 1))) "None" "SnapToTarget" "SnapToTarget" "KeepWorld" true)
        (Variables|/Script/CableComponent.CableComponent|SetCableLength (Variables|/Game/MassiveRoadPack/CityPack/Update/BP_PowerPolesSpline.BP_PowerPolesSpline_C|GetCable2 (Utilities|Array|Get(acopy) _powerpole_array (Variables|Default|GetIndex%20Loop2))) (+ (Math|Vector|VectorLength (- (Transformation|GetWorldLocation (Variables|/Game/MassiveRoadPack/CityPack/Update/BP_PowerPolesSpline.BP_PowerPolesSpline_C|GetConnect2 (Utilities|Array|Get(acopy) _powerpole_array (Variables|Default|GetIndex%20Loop2)))) (Transformation|GetWorldLocation (Variables|/Game/MassiveRoadPack/CityPack/Update/BP_PowerPolesSpline.BP_PowerPolesSpline_C|GetConnect2 (Utilities|Array|Get(acopy) _powerpole_array (+ (Variables|Default|GetIndex%20Loop2) 1)))))) (Math|Random|RandomFloatinRange 0.0 _random_powerline_length)))
        (Variables|/Script/CableComponent.CableComponent|SetCableLength (Variables|/Game/MassiveRoadPack/CityPack/Update/BP_PowerPolesSpline.BP_PowerPolesSpline_C|GetCable2 (Utilities|Array|Get(acopy) (Variables|Default|GetPowerPole%20Array) (Variables|Default|GetNumberOfSplinePoints))) 0.0)))))