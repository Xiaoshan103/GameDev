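; Configurable power pole prop for city scenes, with optional cables, planks, insulators, fuses and coil barrel.
; The construction script uses boolean options to destroy unwanted cable and fuse components, toggle visibility of pole parts, and set live cable lengths.
; A priority chain of version flags swaps the material on the pole and both planks.
; On BeginPlay, it optionally plays a selectable power sound.
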(event EventBeginPlay
  (bind _audio (Variables|Default|GetAudio))
  (if (Variables|Default|GetPlay%20PowerSound?)
    (Audio|Components|Audio|SetSound _audio (Variables|Default|GetSelectSound))
    (Audio|Components|Audio|Play _audio 0.0)))

(fn ConstructionScript
  (bind _mainpole_lp (Variables|Default|GetMainPole_lp))
  (bind _tplank2_lp (Variables|Default|GetTPlank2_lp))
  (bind _tplank_lp (Variables|Default|GetTPlank_lp))
  (bind _mainpole_lp_2 (Variables|Default|GetMainPole_lp))
  (bind _powerbarrel_lp (Variables|Default|GetPowerBarrel_lp))
  (Utilities|FlowControl|Sequence
    (:then_0
      ;[1 1 1] Remove Specific Cables
      (if (not (Variables|CABLES|GetLiveCable1?))
        (Components|DestroyComponent (Variables|Default|GetLiveCable1))))
    (:then_1
      (if (not (Variables|CABLES|GetLiveCable2?))
        (Components|DestroyComponent (Variables|Default|GetLiveCable2))))
    (:then_2
      (if (not (Variables|CABLES|GetLiveConnectCable1?))
        (Components|DestroyComponent (Variables|Default|GetTopFeedCable1))))
    (:then_3
      (if (not (Variables|CABLES|GetLiveConnectCable2?))
        (Components|DestroyComponent (Variables|Default|GetTopFeedCable2))))
    (:then_4
      (if (not (Variables|CABLES|GetLowerFeedCable2?))
        (Components|DestroyComponent (Variables|Default|GetLowerFeedCable2))))
    (:then_5
      (if (not (Variables|CABLES|GetLowerFeedCable1?))
        (Components|DestroyComponent (Variables|Default|GetLowerFeedCable1))))
    (:then_6
      (if (not (Variables|CABLES|GetMiddleFeedCable1?))
        (Components|DestroyComponent (Variables|Default|GetMiddleFeedCable1))))
    (:then_7
      (if (not (Variables|CABLES|GetMiddleFeedCable2?))
        (Components|DestroyComponent (Variables|Default|GetMiddleFeedCable2))))
    (:then_8
      (Utilities|FlowControl|Sequence
        (:then_0
          (Utilities|FlowControl|Sequence
            (:then_0
              ;[1 1 1] Remove Specific Parts
              (if (Variables|POWERPOLEPARTS|GetPowePole)
                (Rendering|SetVisibility _mainpole_lp_2 true false)
                (else
                  (Rendering|SetVisibility _mainpole_lp_2 false false))))
            (:then_1
              (if (Variables|POWERPOLEPARTS|GetPowerCoilBarrel?)
                (Rendering|SetVisibility _powerbarrel_lp true false)
                (else
                  (Rendering|SetVisibility _powerbarrel_lp false false))))
            (:then_2
              (if (Variables|POWERPOLEPARTS|GetUpperPlank?)
                (Rendering|SetVisibility _tplank2_lp true false)
                (else
                  (Rendering|SetVisibility _tplank2_lp false false))))
            (:then_3
              (if (Variables|POWERPOLEPARTS|GetLowerPlank?)
                (Rendering|SetVisibility _tplank_lp true false)
                (else
                  (Rendering|SetVisibility _tplank_lp false false))))
            (:then_4
              (if (not (Variables|POWERPOLEPARTS|GetFuse1?))
                (Components|DestroyComponent (Variables|Default|GetPlate2_lp))))
            (:then_5
              (if (not (Variables|POWERPOLEPARTS|GetFuse2?))
                (Components|DestroyComponent (Variables|Default|GetFuses1_lp))))))
        (:then_1
          (Variables|/Script/CableComponent.CableComponent|SetCableLength (Variables|Default|GetLiveCable2) (Variables|CABLES|GetLiveCable2%20Length)))
        (:then_2
          (Variables|/Script/CableComponent.CableComponent|SetCableLength (Variables|Default|GetLiveCable1) (Variables|CABLES|GetLiveCable1%20Length)))))
    (:then_9
      ;[1 1 1] Alternative Material Selection
      (Utilities|FlowControl|Sequence
        (:then_0
          (if (Variables|PAINT|GetMaterial%20Version2?)
            (Rendering|Material|SetMaterial _mainpole_lp 0 "/Game/MassiveRoadPack/CityPack/Materials/M_PowerPoles2.M_PowerPoles2")
            (elif (Variables|PAINT|GetMaterial%20Version3?)
              (Rendering|Material|SetMaterial _mainpole_lp 0 "/Game/MassiveRoadPack/CityPack/Materials/M_PowerPoles3.M_PowerPoles3")
              (elif (Variables|PAINT|GetMaterial%20Version4?)
                (Rendering|Material|SetMaterial _mainpole_lp 0 "/Game/MassiveRoadPack/CityPack/Materials/M_PowerPoles4.M_PowerPoles4")
                (elif (Variables|PAINT|GetMaterial%20Version5?)
                  (Rendering|Material|SetMaterial _mainpole_lp 0 "/Game/MassiveRoadPack/CityPack/Materials/M_PowerPoles5.M_PowerPoles5"))))))))))