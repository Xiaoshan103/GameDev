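; Configurable traffic light prop with optional pedestrian signals and LED street lamp.
; The construction script selects pole mesh, housing materials, visible parts and lamp lighting, offsetting heads to suit pole height.
; BeginPlay creates dynamic materials, then chained timelines and delays animate emissive power red, green, yellow, and alternate the two pedestrian lights.
; TrafficSignalLoops gates both loops; Timeline_Yellow drives green materials and Timeline_Green drives yellow.
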(event Custom|Event_LightLoop
  (bind _light_off_duration (Variables|TrafficAutomation|GetLight%20OFF%20Duration))
  (bind _light_on_duration (Variables|TrafficAutomation|GetLight%20ON%20Duration))
  ;[1 1 1] Traffic Lights Operation
  (if (Variables|TrafficAutomation|GetTrafficSignal%20Loops?)
    (bind _newtrack_0 (Timeline|Timeline_RED PlayFromStart)
      (:Update
        (Rendering|Material|SetScalarParameterValue (Variables|Default|GetLightExtendedRed) "EmissiveLightTexturePower" _newtrack_0 :!class /Script/Engine.MaterialInstanceDynamic))
      (:Finished
        (Utilities|FlowControl|Delay _light_off_duration)
        (Components|Timeline|SetPlayRate (Variables|Default|GetTimeline_Yellow) _light_on_duration)
        (bind _newtrack_0_2 (Timeline|Timeline_Yellow PlayFromStart)
          (:Update
            (Rendering|Material|SetScalarParameterValue (Variables|Default|GetLightGreen) "EmissiveLightTexturePower" _newtrack_0_2 :!class /Script/Engine.MaterialInstanceDynamic))
          (:Finished
            (Utilities|FlowControl|Delay _light_off_duration)
            (Components|Timeline|SetPlayRate (Variables|Default|GetTimeline_Green) (* _light_on_duration 3.0))
            (bind _newtrack_0_3 (Timeline|Timeline_Green PlayFromStart)
              (:Update
                (Rendering|Material|SetScalarParameterValue (Variables|Default|GetLightYellow) "EmissiveLightTexturePower" _newtrack_0_3 :!class /Script/Engine.MaterialInstanceDynamic))
              (:Finished
                (Utilities|FlowControl|Delay _light_off_duration)
                (CallFunction|EventLightLoop)))))))))

(event Custom|Event_PedestrianLoop
  (bind _pedestrianlights_off_duration (Variables|TrafficAutomation|GetPedestrianLights%20OFF%20Duration))
  ;[1 1 1] Comment
  (if (Variables|TrafficAutomation|GetTrafficSignal%20Loops?)
    (bind _newtrack_0 (Timeline|Timeline_Pedestrian1 PlayFromStart)
      (:Update
        (Rendering|Material|SetScalarParameterValue (Variables|Default|GetPedestrianLightDyn) "EmissivePower" _newtrack_0 :!class /Script/Engine.MaterialInstanceDynamic))
      (:Finished
        (Utilities|FlowControl|Delay _pedestrianlights_off_duration)
        (Components|Timeline|SetPlayRate (Variables|Default|GetTimeline_Pedestrian2) (Variables|TrafficAutomation|GetPedestrianLights%20ON%20Duration))
        (bind _newtrack_0_2 (Timeline|Timeline_Pedestrian2 PlayFromStart)
          (:Update
            (Rendering|Material|SetScalarParameterValue (Variables|Default|GetPedestrianLightDyn2) "EmissivePower" _newtrack_0_2 :!class /Script/Engine.MaterialInstanceDynamic))
          (:Finished
            (Utilities|FlowControl|Delay _pedestrianlights_off_duration)
            (CallFunction|EventPedestrianLoop)))))))

(event EventBeginPlay
  (bind _pedestrianlights_on_duration (Variables|TrafficAutomation|GetPedestrianLights%20ON%20Duration))
  (bind _light_off_duration (Variables|TrafficAutomation|GetLight%20OFF%20Duration))
  (bind _light_on_duration (Variables|TrafficAutomation|GetLight%20ON%20Duration))
  (bind _pedestrianlights_off_duration (Variables|TrafficAutomation|GetPedestrianLights%20OFF%20Duration))
  (bind _trafficlightextended (Variables|Default|GetTrafficLightExtended))
  (bind _trafficlight (Variables|Default|GetTrafficLight))
  (bind _pedestrianlight2 (Variables|Default|GetPedestrianLight2))
  (bind _pedestrianlight1 (Variables|Default|GetPedestrianLight1))
  (Utilities|FlowControl|Sequence
    (:then_0
      (if (Variables|TrafficAutomation|GetTrafficSignal%20Operating?)
        ;[1 1 1] Creating Dynamic Materials
        (Utilities|FlowControl|Sequence
          (:then_0
            (if true
              (Utilities|FlowControl|Sequence
                (:then_0
                  (bind _returnvalue (Rendering|Material|CreateDynamicMaterialInstance _trafficlightextended 1 (Rendering|Material|GetMaterial _trafficlightextended 1) :!class /Script/Engine.PrimitiveComponent))
                  (Variables|Default|SetLightExtendedRed _returnvalue))
                (:then_1
                  (bind _returnvalue_2 (Rendering|Material|CreateDynamicMaterialInstance _trafficlightextended 2 (Rendering|Material|GetMaterial _trafficlightextended 2) :!class /Script/Engine.PrimitiveComponent))
                  (Variables|Default|SetLightExtendedYellow _returnvalue_2))
                (:then_2
                  (bind _returnvalue_3 (Rendering|Material|CreateDynamicMaterialInstance _trafficlightextended 3 (Rendering|Material|GetMaterial _trafficlightextended 3) :!class /Script/Engine.PrimitiveComponent))
                  (Variables|Default|SetLightExtendedGreen _returnvalue_3)))))
          (:then_1
            (if true
              (Utilities|FlowControl|Sequence
                (:then_0
                  (bind _returnvalue_4 (Rendering|Material|CreateDynamicMaterialInstance _trafficlight 1 (Rendering|Material|GetMaterial _trafficlight 1) :!class /Script/Engine.PrimitiveComponent))
                  (Variables|Default|SetLightRed _returnvalue_4))
                (:then_1
                  (bind _returnvalue_5 (Rendering|Material|CreateDynamicMaterialInstance _trafficlight 2 (Rendering|Material|GetMaterial _trafficlight 2) :!class /Script/Engine.PrimitiveComponent))
                  (Variables|Default|SetLightYellow _returnvalue_5))
                (:then_2
                  (bind _returnvalue_6 (Rendering|Material|CreateDynamicMaterialInstance _trafficlight 3 (Rendering|Material|GetMaterial _trafficlight 3) :!class /Script/Engine.PrimitiveComponent))
                  (Variables|Default|SetLightGreen _returnvalue_6)))))
          (:then_2
            ;[1 1 1] Traffic Lights Operation
            (Utilities|FlowControl|Delay (Variables|TrafficAutomation|GetTrafficStartDelay))
            (Components|Timeline|SetPlayRate (Variables|Default|GetTimeline_RED) _light_on_duration)
            (bind _newtrack_0 (Timeline|Timeline_RED PlayFromStart)
              (:Update
                (Rendering|Material|SetScalarParameterValue (Variables|Default|GetLightExtendedRed) "EmissiveLightTexturePower" _newtrack_0 :!class /Script/Engine.MaterialInstanceDynamic))
              (:Finished
                (Utilities|FlowControl|Delay _light_off_duration)
                (Components|Timeline|SetPlayRate (Variables|Default|GetTimeline_Yellow) _light_on_duration)
                (bind _newtrack_0_2 (Timeline|Timeline_Yellow PlayFromStart)
                  (:Update
                    (Rendering|Material|SetScalarParameterValue (Variables|Default|GetLightGreen) "EmissiveLightTexturePower" _newtrack_0_2 :!class /Script/Engine.MaterialInstanceDynamic))
                  (:Finished
                    (Utilities|FlowControl|Delay _light_off_duration)
                    (Components|Timeline|SetPlayRate (Variables|Default|GetTimeline_Green) (* _light_on_duration 3.0))
                    (bind _newtrack_0_3 (Timeline|Timeline_Green PlayFromStart)
                      (:Update
                        (Rendering|Material|SetScalarParameterValue (Variables|Default|GetLightYellow) "EmissiveLightTexturePower" _newtrack_0_3 :!class /Script/Engine.MaterialInstanceDynamic))
                      (:Finished
                        (Utilities|FlowControl|Delay _light_off_duration)
                        (CallFunction|EventLightLoop)))))))))))
    (:then_1
      ;[1 1 1] Comment
      (if (Variables|TrafficAutomation|GetPedestrianLights%20Operating?)
        (Utilities|FlowControl|Sequence
          (:then_0
            (Utilities|FlowControl|Sequence
              (:then_0
                (bind _returnvalue_7 (Rendering|Material|CreateDynamicMaterialInstance _pedestrianlight1 1 (Rendering|Material|GetMaterial _pedestrianlight1 1) :!class /Script/Engine.PrimitiveComponent))
                (Variables|Default|SetPedestrianLightDyn _returnvalue_7))
              (:then_1
                (bind _returnvalue_8 (Rendering|Material|CreateDynamicMaterialInstance _pedestrianlight2 1 (Rendering|Material|GetMaterial _pedestrianlight2 1) :!class /Script/Engine.PrimitiveComponent))
                (Variables|Default|SetPedestrianLightDyn2 _returnvalue_8))))
          (:then_1
            (Utilities|FlowControl|Delay (Variables|TrafficAutomation|GetPedestrianLights%20StartDelay))
            (Components|Timeline|SetPlayRate (Variables|Default|GetTimeline_Pedestrian1) _pedestrianlights_on_duration)
            (bind _newtrack_0_4 (Timeline|Timeline_Pedestrian1 PlayFromStart)
              (:Update
                (Rendering|Material|SetScalarParameterValue (Variables|Default|GetPedestrianLightDyn) "EmissivePower" _newtrack_0_4 :!class /Script/Engine.MaterialInstanceDynamic))
              (:Finished
                (Utilities|FlowControl|Delay _pedestrianlights_off_duration)
                (Components|Timeline|SetPlayRate (Variables|Default|GetTimeline_Pedestrian2) _pedestrianlights_on_duration)
                (bind _newtrack_0_5 (Timeline|Timeline_Pedestrian2 PlayFromStart)
                  (:Update
                    (Rendering|Material|SetScalarParameterValue (Variables|Default|GetPedestrianLightDyn2) "EmissivePower" _newtrack_0_5 :!class /Script/Engine.MaterialInstanceDynamic))
                  (:Finished
                    (Utilities|FlowControl|Delay _pedestrianlights_off_duration)
                    (CallFunction|EventPedestrianLoop)))))))))))

(fn ConstructionScript
  (bind _streetlampled (Variables|Default|GetStreetLampLED))
  (bind _streetlampled_2 (Variables|Default|GetStreetLampLED))
  (Utilities|FlowControl|Sequence
    (:then_0
      ;[1 1 1] Set Alternative Material
      (if (Variables|Paint|GetMainLightBlack?)
        (Rendering|Material|SetMaterial (Variables|Default|GetTrafficLight) 0 "/Game/MassiveRoadPack/CityPack/Materials/M_TrafficLights_Base2.M_TrafficLights_Base2")))
    (:then_1
      (if (Variables|Paint|GetPedestrianLightYellow?)
        (Rendering|Material|SetMaterial (Variables|Default|GetPedestrianLight2) 0 "/Game/MassiveRoadPack/CityPack/Materials/M_TrafficLight_Pedestrian_Inst2.M_TrafficLight_Pedestrian_Inst2")))
    (:then_2
      ;[1 1 1] Asset Parts Selection
      (if (Variables|Default|GetPole%208FT?)
        (|PoleMeshSelector (Variables|Default|GetPole) :!label _label
          (:TrueOutput
            ;;[0.439 1 0.4515] Resets Position based off selection
            (Utilities|FlowControl|Sequence
              (:then_0
                (Utilities|FlowControl|DoOnce false :!label _label_2
                  (:Completed
                    (Transformation|AddLocalOffset (Variables|Default|GetTrafficLight) "-213.000000, 0, 0" false false)
                    (Transformation|AddLocalOffset _streetlampled "0.000000,-213.000000, 0" false false))))
              (:then_1
                (if (not (Variables|Default|GetPole%208FT?))
                  (goto _label_2 Reset)))))
          (:FalseOutput
            (Utilities|FlowControl|Sequence
              (:then_0
                (Utilities|FlowControl|DoOnce true :!label _label_3
                  (:Completed
                    (Transformation|AddLocalOffset (Variables|Default|GetTrafficLightExtended) "213.000000, 0, 0" false false)
                    (Transformation|AddLocalOffset _streetlampled "0.000000,213.000000, 0" false false))))
              (:then_1
                (if (Variables|Default|GetPole%208FT?)
                  (goto _label_3 Reset))))))
        (else
          (goto _label False))))
    (:then_3
      (if (Variables|Default|GetTrafficLightBasic?)
        (Rendering|SetVisibility (Variables|Default|GetTrafficLight) true false)
        (elif (Variables|Default|GetTrafficLightExtended%20Version?)
          (Rendering|SetVisibility (Variables|Default|GetTrafficLightExtended) true false))))
    (:then_5
      (Rendering|SetVisibility (Variables|Default|GetStreetLampLED) (Variables|StreetLamp|GetStreetLamp?) false)
      ;;[0.439 1 0.4515] Sets Street Lamp Fucntionality
      (if (Variables|StreetLamp|GetStreetLamp?)
        (Utilities|FlowControl|Sequence
          (:then_0
            (Rendering|SetVisibility (Variables|Default|GetSpotLight) (Variables|StreetLamp|GetStreetLamp%20ON?) false)
            (bind _returnvalue (Rendering|Material|CreateDynamicMaterialInstance _streetlampled_2 0 (Rendering|Material|GetMaterial _streetlampled_2 1) :!class /Script/Engine.PrimitiveComponent))
            (bind _output_get (Variables|Default|SetLightStreet _returnvalue))
            (Rendering|Material|SetScalarParameterValue _output_get "EmissivePower" (Variables|StreetLamp|GetStreetLampGlow) :!class /Script/Engine.MaterialInstanceDynamic))
          (:then_1
            (Rendering|SetVisibility (Variables|Default|GetPointLight) (Variables|StreetLamp|GetStreetLampAmbience%20ON?) false))
          (:then_3
            (if (not (or (Variables|StreetLamp|GetStreetLamp%20ON?) (Variables|StreetLamp|GetStreetLampAmbience%20ON?)))
              (Rendering|Material|SetScalarParameterValue _output_get "EmissivePower" 0.0 :!class /Script/Engine.MaterialInstanceDynamic))))))
    (:then_6
      (Rendering|SetVisibility (Variables|Default|GetPedestrianLight1) (Variables|Default|GetPesdestrianLight1?) false))
    (:then_7
      (Rendering|SetVisibility (Variables|Default|GetPedestrianLight2) (Variables|Default|GetPesdestrianLight2?) false))))