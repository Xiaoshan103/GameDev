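; Configurable road sign Blueprint for stop, assorted, construction and speed signs, assembled entirely in the construction script.
; Pole flags choose wood, round steel, angular steel or no pole with matching bolts, then height, scale and rotation are applied.
; A sign category enum and option index drive Select nodes for mesh visibility and material, with colored number text for speed signs.
; A custom sign flag instead assigns a user-chosen mesh and optional material.
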(fn ConstructionScript
  (bind _textrender (Variables|Default|GetTextRender))
  (bind _select_sign_type (Variables|SignTypeSelection|GetSelect%20Sign%20Type))
  (bind _diamond_sign (Variables|Default|GetDIAMOND_SIGN))
  (bind _select_sign_type_2 (Variables|SignTypeSelection|GetSelect%20Sign%20Type))
  (bind _stop_sign (Variables|Default|GetSTOP_SIGN))
  (bind _signs (Variables|Default|GetSigns))
  (bind _tall_smooth_sign (Variables|Default|GetTALL_SMOOTH_SIGN))
  (bind _signscale (Variables|SignTransformations|GetSignScale))
  (bind _vertical_sign (Variables|Default|GetVERTICAL_SIGN))
  (bind _select_sign_type_3 (Variables|SignTypeSelection|GetSelect%20Sign%20Type))
  (bind _small_sharp_sign (Variables|Default|GetSMALL_SHARP_SIGN))
  (bind _select_sign_type_4 (Variables|SignTypeSelection|GetSelect%20Sign%20Type))
  (bind _customsignref (Variables|Default|GetCustomSignRef))
  (bind _returnvalue (* 1.0 _signscale))
  (bind _returnvalue_2 (Utilities|Select :Index _select_sign_type :Option%200 _diamond_sign :Option%201 _diamond_sign :Option%202 _diamond_sign :Option%203 _diamond_sign :Option%204 _diamond_sign :Option%205 _diamond_sign :Option%206 _diamond_sign :Option%207 _diamond_sign :Option%208 _diamond_sign :Option%209 _diamond_sign :Option%2010 _diamond_sign :Option%2011 _diamond_sign))
  (bind _returnvalue_3 (Utilities|Select :Index _select_sign_type_2 :Option%200 _stop_sign :Option%201 _stop_sign))
  (bind _returnvalue_4 (Utilities|Select :Index _select_sign_type_4 :Option%200 _tall_smooth_sign :Option%201 _tall_smooth_sign))
  (bind _returnvalue_5 (Utilities|Select :Index _select_sign_type_3 :Option%200 _vertical_sign :Option%201 _vertical_sign :Option%202 _vertical_sign :Option%203 _small_sharp_sign :Option%204 _small_sharp_sign))
  (Utilities|FlowControl|Sequence
    (:then_0
      ;[1 1 1] Set SignPole
      (if (Variables|SignPoleSelection|GetSignPole%20Wood?)
        (Rendering|SetVisibility (Variables|Default|GetWOODPOLE) true false)
        (Rendering|SetVisibility (Variables|Default|GetROUNDPOLE) false false)
        (Variables|SignPoleSelection|SetSignPole%20SteelRound? false)
        (Variables|SignPoleSelection|SetSignPole%20SteelAngular? false)
        ;[1 1 1] Set SignPole Bolts
        (Rendering|SetVisibility (Variables|Default|GetWOODPOLEBolts) true false)
        (Rendering|SetVisibility (Variables|Default|GetROUNDPOLEBolts) false false)
        (Rendering|SetVisibility (Variables|Default|GetSIGNPOLEBolts) false false)
        (elif (Variables|SignPoleSelection|GetSignPole%20SteelRound?)
          (Rendering|SetVisibility (Variables|Default|GetROUNDPOLE) true false)
          (Rendering|SetVisibility (Variables|Default|GetWOODPOLE) false false)
          (Variables|SignPoleSelection|SetSignPole%20Wood? false)
          (Variables|SignPoleSelection|SetSignPole%20SteelAngular? false)
          (Rendering|SetVisibility (Variables|Default|GetROUNDPOLEBolts) true false)
          (Rendering|SetVisibility (Variables|Default|GetWOODPOLEBolts) false false)
          (Rendering|SetVisibility (Variables|Default|GetSIGNPOLEBolts) false false)
          (elif (Variables|SignPoleSelection|GetSignPole%20SteelAngular?)
            (Rendering|SetVisibility (Variables|Default|GetSIGNPOLE) true false)
            (Rendering|SetVisibility (Variables|Default|GetWOODPOLE) false false)
            (Variables|SignPoleSelection|SetSignPole%20Wood? false)
            (Variables|SignPoleSelection|SetSignPole%20SteelRound? false)
            (Rendering|SetVisibility (Variables|Default|GetSIGNPOLEBolts) true false)
            (Rendering|SetVisibility (Variables|Default|GetWOODPOLEBolts) false false)
            (Rendering|SetVisibility (Variables|Default|GetROUNDPOLEBolts) false false)
            (elif (Variables|SignPoleSelection|GetSignPole%20Removed?)
              (Rendering|SetVisibility (Variables|Default|GetWOODPOLE) false false)
              (Variables|SignTransformations|SetSign%20Height 0.0)
              (Variables|SignPoleSelection|SetSignPole%20Wood? false)
              (Variables|SignPoleSelection|SetSignPole%20SteelAngular? false)
              (Variables|SignPoleSelection|SetSignPole%20SteelRound? false)
              (Rendering|SetVisibility (Variables|Default|GetWOODPOLEBolts) false false))))))
    (:then_1
      ;[1 1 1] Set Custom Sign
      (if (Variables|CustomSign|GetCustomSign?)
        (Components|StaticMesh|SetStaticMesh _customsignref (Variables|CustomSign|GetSelect%20CustomSign))
        (if (Variables|CustomSign|GetCustomMaterial?)
          (Rendering|Material|SetMaterial _customsignref 0 (Variables|CustomSign|GetSelect%20CustomSign%20Material)))))
    (:then_5
      ;[1 1 1] Set Sign+bolt Location
      (Transformation|AddRelativeLocation (Variables|Default|GetBolts) (Math|Vector|MakeVector 0.0 0.0 (Variables|SignTransformations|GetSign%20Height)) false false))
    (:then_6
      ;[1 1 1] Set Sign Scale + Rotation
      (Transformation|SetWorldScale3D _signs (Math|Vector|MakeVector _returnvalue 1.0 _returnvalue))
      (Transformation|SetRelativeRotation _signs (Math|Rotator|MakeRotator 0.0 (Variables|SignTransformations|GetSign%20Rotation) 0.0) false false))
    (:then_8
      (if (not (Variables|CustomSign|GetCustomSign?))
        (Utilities|FlowControl|Sequence
          (:then_0
            ;[1 1 1] Speed Controls
            (Utilities|FlowControl|Sequence
              (:then_0
                (if (Utilities|Select :Index (Variables|SignTypeSelection|GetSign%20Type%20Selector) :NewEnumerator0 false :NewEnumerator8 false :NewEnumerator1 false :NewEnumerator2 true)
                  (Rendering|SetVisibility _textrender true false)
                  (else
                    (Rendering|SetVisibility _textrender false false))))
              (:then_1
                (Rendering|Components|TextRender|SetText _textrender (Utilities|Text|ToText(Integer) (Variables|SignTypeSelection|GetSpeed%20Number))))
              (:then_2
                (Rendering|Components|TextRender|SetTextRenderColor _textrender (Math|Conversions|ToColor(LinearColor) (Variables|SignTypeSelection|GetSpeed%20Color))))))
          (:then_1
            ;[1 1 1] Stop Sign Selector
            ;;[1 0.3041 0.07268] Select Sign Type
            (if (Utilities|Select :Index (Variables|SignTypeSelection|GetSign%20Type%20Selector) :NewEnumerator0 true :NewEnumerator8 false :NewEnumerator1 false :NewEnumerator2 false)
              ;;[1 0.3041 0.07268] Set StaticMesh Options
              (Rendering|SetVisibility _returnvalue_3 true false)
              ;;[1 0.3041 0.07268] Set Material Options
              (Rendering|Material|SetMaterial _returnvalue_3 1 (Utilities|Select :Index _select_sign_type_2 :Option%200 (Variables|CustomSign|GetSelect%20CustomSign%20Material) :Option%201 "/Game/MassiveRoadPack/SharedAssets/Materials/M_Stop_Sign_Inst.M_Stop_Sign_Inst"))
              (else
                (Utilities|FlowControl|Sequence
                  (:then_0
                    (Rendering|SetVisibility _returnvalue_3 false false))
                  (:then_1
                    ;[1 1 1] Assorted Signs
                    ;;[1 0.3041 0.07268] Select Sign Type
                    (if (Utilities|Select :Index (Variables|SignTypeSelection|GetSign%20Type%20Selector) :NewEnumerator0 false :NewEnumerator8 true :NewEnumerator1 false :NewEnumerator2 false)
                      ;;[1 0.3041 0.07268] Set StaticMesh Options
                      (Rendering|SetVisibility _returnvalue_5 true false)
                      ;;[1 0.3041 0.07268] Set Material Options
                      (Rendering|Material|SetMaterial _returnvalue_5 0 (Utilities|Select :Index _select_sign_type_3 :Option%200 (Variables|CustomSign|GetSelect%20CustomSign%20Material) :Option%201 "/Game/MassiveRoadPack/SharedAssets/Materials/M_Vertical_Sign_Inst.M_Vertical_Sign_Inst" :Option%202 "/Game/MassiveRoadPack/SharedAssets/Materials/M_Vertical_Sign_Inst1.M_Vertical_Sign_Inst1" :Option%203 "/Game/MassiveRoadPack/SharedAssets/Materials/M_Vertical_Sign_Inst2.M_Vertical_Sign_Inst2" :Option%204 "/Game/MassiveRoadPack/SharedAssets/Materials/M_Vertical_Sign_Inst3.M_Vertical_Sign_Inst3"))
                      (else
                        (Utilities|FlowControl|Sequence
                          (:then_0
                            (Rendering|SetVisibility _returnvalue_5 false false))
                          (:then_1
                            ;[1 1 1] Constructions Signs
                            ;;[1 0.3041 0.07268] Select Sign Type
                            (if (Utilities|Select :Index (Variables|SignTypeSelection|GetSign%20Type%20Selector) :NewEnumerator0 false :NewEnumerator8 false :NewEnumerator1 true :NewEnumerator2 false)
                              ;;[1 0.3041 0.07268] Add StaticMesh Options
                              (Rendering|SetVisibility _returnvalue_2 true false)
                              ;;[1 0.3041 0.07268] Add Material Options
                              (Rendering|Material|SetMaterial _returnvalue_2 0 (Utilities|Select :Index _select_sign_type :Option%200 (Variables|CustomSign|GetSelect%20CustomSign%20Material) :Option%201 "/Game/MassiveRoadPack/SharedAssets/Materials/M_Diamond_Sign_Master_Inst.M_Diamond_Sign_Master_Inst" :Option%202 "/Game/MassiveRoadPack/SharedAssets/Materials/M_Diamond_Sign_Master_Inst0.M_Diamond_Sign_Master_Inst0" :Option%203 "/Game/MassiveRoadPack/SharedAssets/Materials/M_Diamond_Sign_Master_Inst1.M_Diamond_Sign_Master_Inst1" :Option%204 "/Game/MassiveRoadPack/SharedAssets/Materials/M_Diamond_Sign_Master_Inst2.M_Diamond_Sign_Master_Inst2" :Option%205 "/Game/MassiveRoadPack/SharedAssets/Materials/M_Diamond_Sign_Master_Inst3.M_Diamond_Sign_Master_Inst3" :Option%206 "/Game/MassiveRoadPack/SharedAssets/Materials/M_Diamond_Sign_Master_Inst4.M_Diamond_Sign_Master_Inst4" :Option%207 "/Game/MassiveRoadPack/SharedAssets/Materials/M_Diamond_Sign_Master_Inst5.M_Diamond_Sign_Master_Inst5" :Option%208 "/Game/MassiveRoadPack/SharedAssets/Materials/M_Diamond_Sign_Master_Inst6.M_Diamond_Sign_Master_Inst6" :Option%209 "/Game/MassiveRoadPack/SharedAssets/Materials/M_Diamond_Sign_Master_Inst7.M_Diamond_Sign_Master_Inst7" :Option%2010 "/Game/MassiveRoadPack/SharedAssets/Materials/M_Diamond_Sign_Master_Inst8.M_Diamond_Sign_Master_Inst8" :Option%2011 "/Game/MassiveRoadPack/SharedAssets/Materials/M_Diamond_Sign_Master_Inst9.M_Diamond_Sign_Master_Inst9"))
                              (else
                                (Utilities|FlowControl|Sequence
                                  (:then_0
                                    (Rendering|SetVisibility _returnvalue_2 false false))
                                  (:then_1
                                    ;[1 1 1] Speed Signs
                                    ;;[1 0.3041 0.07268] Select Sign Type
                                    (if (Utilities|Select :Index (Variables|SignTypeSelection|GetSign%20Type%20Selector) :NewEnumerator0 false :NewEnumerator8 false :NewEnumerator1 false :NewEnumerator2 true)
                                      ;;[1 0.3041 0.07268] Add StaticMesh Options
                                      (Rendering|SetVisibility _returnvalue_4 true false)
                                      ;;[1 0.3041 0.07268] Add Material Options
                                      (Rendering|Material|SetMaterial _returnvalue_4 1 (Utilities|Select :Index _select_sign_type_4 :Option%200 (Variables|CustomSign|GetSelect%20CustomSign%20Material) :Option%201 "/Game/MassiveRoadPack/SharedAssets/Materials/M_Speed_Sign_Inst1.M_Speed_Sign_Inst1"))
                                      (else
                                        (Utilities|FlowControl|Sequence
                                          (:then_0
                                            (Rendering|SetVisibility _returnvalue_4 false false)))))))))))))))))))))))