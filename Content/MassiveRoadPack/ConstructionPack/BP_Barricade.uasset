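; BP_Barricade is a configurable construction barricade prop with a connecting rail, two legs and a reflector.
; Its construction script checks a boolean for each part and toggles that component's visibility when the matching Remove option is set, letting each placed instance omit pieces.
; The event graph holds only disabled placeholder events, so the asset has no gameplay logic.
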(event EventBeginPlay)

(event Collision|EventActorBeginOverlap
  (params (OtherActor :type Actor%20Object%20Reference)))

(event EventTick
  (params (DeltaSeconds :type Float%20%28single-precision%29)))

(fn ConstructionScript
  (Utilities|FlowControl|Sequence
    (:then_0
      (if (Variables|Default|GetRemove%20ConnectingRod)
        (Utilities|FlowControl|FlipFlop
          (:A
            _)
          (:B
            _))
        (Rendering|ToggleVisibility (Variables|Default|GetConnectingRail) false)))
    (:then_1
      (if (Variables|Default|GetRemove%20Leg1)
        (Utilities|FlowControl|FlipFlop
          (:A
            _)
          (:B
            _))
        (Rendering|ToggleVisibility (Variables|Default|GetBarricade_Leg1) false)))
    (:then_2
      (if (Variables|Default|GetRemove%20Leg2)
        (Utilities|FlowControl|FlipFlop
          (:A
            _)
          (:B
            _))
        (Rendering|ToggleVisibility (Variables|Default|GetBarricade_Leg2) false)))
    (:then_3
      (if (Variables|Default|GetRemove%20Reflector)
        (Utilities|FlowControl|FlipFlop
          (:A
            _)
          (:B
            _))
        (Rendering|ToggleVisibility (Variables|Default|GetReflector) false)))))