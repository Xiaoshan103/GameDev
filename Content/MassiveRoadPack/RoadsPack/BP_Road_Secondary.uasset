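; BP_Road_Secondary is a spline-driven road builder that generates its meshes in the Construction Script, with no active runtime logic.
; It resizes a per-point data array to match the spline, supplying width, thickness, bank and guard-rail toggles.
; A loop macro feeds each segment to BuildTrackElement, adding spline meshes for road and left/right rails, wrapping to the first point for closed loops.
; Optional text renders number the spline points.
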(event EventBeginPlay)

(event Collision|EventActorBeginOverlap
  (params (OtherActor :type Actor%20Object%20Reference)))

(event EventTick
  (params (DeltaSeconds :type Float%20%28single-precision%29)))

(fn ConstructionScript
  (Utilities|FlowControl|Sequence
    (:then_0
      (|StoreNumberOFSplinePoints))
    (:then_1
      (|BuildRoadDataArray))
    (:then_2
      (|ConstructionLoop)
      (|StoreDrawGuardRails)
      (Utilities|FlowControl|Sequence
        (:then_0
          (if (Variables|SplineMeshes|GetDraw%20RoadMesh?)
            (CallFunction|BuildTrackElement (Variables|Default|GetCurrentLoopIndex) (Variables|SplineMeshes|GetRoadMesh))))
        (:then_1
          (if (Variables|Default|GetDraw%20Left%20Guard%20Rail)
            (CallFunction|BuildTrackElement (Variables|Default|GetCurrentLoopIndex) (Variables|SplineMeshes|GetLeftGuardRail))))
        (:then_2
          (if (Variables|Default|GetDraw%20Right%20Guard%20Rail)
            (CallFunction|BuildTrackElement (Variables|Default|GetCurrentLoopIndex) (Variables|SplineMeshes|GetRightGuardRail))))))
    (:then_3
      (|DrawSplinePointNumbers))))

(fn BuildTrackElement
  (params (LoopIndex :type Integer) (TrackElement :type Static%20Mesh%20Object%20Reference))
  (bind _local_startoffset (LocalVariables|GetLocal_StartOffset))
  (bind _spline (Variables|Default|GetSpline))
  (LocalVariables|SetLocal_CurrentLoopIndex LoopIndex)
  (LocalVariables|SetLocal_NextLoopIndex (Math|Integer|%(Integer) (+ LoopIndex 1) (Variables|Default|GetNumberOfSplinePoints)))
  (LocalVariables|SetLocal_TrackElementMesh TrackElement)
  (Utilities|FlowControl|Sequence
    (:then_0
      (LocalVariables|SetLocal_StartLocation (+ (.Location (Spline|GetLocationandTangentatSplinePoint _spline (LocalVariables|GetLocal_CurrentLoopIndex) "Local")) (+ (Class|SplineComponent|GetDirectionatSplinePoint _spline 0 "Local") _local_startoffset)))
      (LocalVariables|SetLocal_StartTangent (+ (.Tangent (Spline|GetLocationandTangentatSplinePoint _spline (LocalVariables|GetLocal_CurrentLoopIndex) "Local")) (+ (Class|SplineComponent|GetDirectionatSplinePoint _spline 0 "Local") _local_startoffset)))
      (LocalVariables|SetLocal_EndLocation (+ (.Location (Spline|GetLocationandTangentatSplinePoint (Variables|Default|GetSpline) (LocalVariables|GetLocal_NextLoopIndex) "Local")) (Variables|Default|GetOffSet)))
      (LocalVariables|SetLocal_EndTangent (+ (.Tangent (Spline|GetLocationandTangentatSplinePoint (Variables|Default|GetSpline) (LocalVariables|GetLocal_NextLoopIndex) "Local")) "0, 0, 0"))
      (LocalVariables|SetLocal_StartRoll (.trackbank (Utilities|Array|Get(acopy) (Variables|Default|GetRoadDataArray) (LocalVariables|GetLocal_CurrentLoopIndex))))
      (LocalVariables|SetLocal_StartScale (Math|Vector2D|MakeVector2D (.trackwidth (Utilities|Array|Get(acopy) (Variables|Default|GetRoadDataArray) (LocalVariables|GetLocal_CurrentLoopIndex))) (.trackthickness (Utilities|Array|Get(acopy) (Variables|Default|GetRoadDataArray) (LocalVariables|GetLocal_CurrentLoopIndex)))))
      (LocalVariables|SetLocal_EndRoll (.trackbank (Utilities|Array|Get(acopy) (Variables|Default|GetRoadDataArray) (LocalVariables|GetLocal_NextLoopIndex))))
      (LocalVariables|SetLocal_EndScale (Math|Vector2D|MakeVector2D (.trackwidth (Utilities|Array|Get(acopy) (Variables|Default|GetRoadDataArray) (LocalVariables|GetLocal_NextLoopIndex))) (.trackthickness (Utilities|Array|Get(acopy) (Variables|Default|GetRoadDataArray) (LocalVariables|GetLocal_NextLoopIndex))))))
    (:then_1
      (bind _returnvalue (AddComponent|AddSplineMeshComponent false))
      (LocalVariables|SetLocal_CurrentSplineMesh _returnvalue)
      (Components|StaticMesh|SetStaticMesh (LocalVariables|GetLocal_CurrentSplineMesh) (LocalVariables|GetLocal_TrackElementMesh))
      (Rendering|Material|SetMaterial (LocalVariables|GetLocal_CurrentSplineMesh) 0 (Variables|SplineMeshes|GetSelect%20Custom%20Road%20Material))
      (SplineMesh|SetStartandEnd (LocalVariables|GetLocal_CurrentSplineMesh) (LocalVariables|GetLocal_StartLocation) (LocalVariables|GetLocal_StartTangent) (LocalVariables|GetLocal_EndLocation) (LocalVariables|GetLocal_EndTangent) true :!class /Script/Engine.SplineMeshComponent)
      (Class|SplineMeshComponent|SetStartRoll (LocalVariables|GetLocal_CurrentSplineMesh) (LocalVariables|GetLocal_StartRoll) true)
      (Class|SplineMeshComponent|SetEndRoll (LocalVariables|GetLocal_CurrentSplineMesh) (LocalVariables|GetLocal_EndRoll) true)
      (SplineMesh|SetStartScale (LocalVariables|GetLocal_CurrentSplineMesh) (LocalVariables|GetLocal_StartScale) true :!class /Script/Engine.SplineMeshComponent)
      (SplineMesh|SetEndScale (LocalVariables|GetLocal_CurrentSplineMesh) (LocalVariables|GetLocal_EndScale) true :!class /Script/Engine.SplineMeshComponent)
      (Collision|SetCollisionEnabled (LocalVariables|GetLocal_CurrentSplineMesh) (Variables|Default|GetCollison?))
      (SplineMesh|SetForwardAxis (LocalVariables|GetLocal_CurrentSplineMesh) (Variables|SplineMeshes|GetRoadMeshAxis) true))))