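; BP_Mergers is a configurable road merge piece that offers city curb, sidewalk, highway and single-lane variants.
; The construction script shows and enables collision on the mesh for the first true Intersection flag, and records its index in IntersectionSelect.
; FlipMirror mirrors the merge meshes through negative Y scale.
; The index then picks the mesh whose start, end and merge sockets the AttachRoad components snap to.
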(fn ConstructionScript
  (bind _sm_road_citycurb_merge (Variables|Default|GetSM_Road_CityCurb_Merge))
  (bind _sm_road_citycurb_x2l_merge (Variables|Default|GetSM_Road_CityCurb_X2L_Merge))
  (bind _sm_road_citycurbwalk_merge (Variables|Default|GetSM_Road_CityCurbWalk_Merge))
  (bind _sm_road_citycurbwalk_x2l_merge (Variables|Default|GetSM_Road_CityCurbWalk_X2L_Merge))
  (bind _sm_road_highway_merge (Variables|Default|GetSM_Road_Highway_Merge))
  (bind _sm_road_highway_x2l_merge (Variables|Default|GetSM_Road_Highway_X2L_Merge))
  (bind _sm_road_singlelane_merge (Variables|Default|GetSM_Road_SingleLane_Merge))
  (Utilities|FlowControl|Sequence
    (:then_0
      ;[1 1 1] Selection Process
      (if (Variables|Default|GetIntersection%20Curb?)
        (Rendering|SetVisibility _sm_road_citycurb_merge true false)
        (Collision|SetCollisionEnabled _sm_road_citycurb_merge "QueryAndPhysics")
        (Variables|Default|SetIntersectionSelect 1)
        (if (Variables|Default|GetFlip/Mirror?) :!label _label
          (Transformation|SetWorldScale3D (Variables|Default|GetSM_Road_CityCurb_X2L_Merge) "1.000000,-1.000000,1.000000"))
        (elif (Variables|Default|GetIntersection%20CurbX2?)
          (Rendering|SetVisibility _sm_road_citycurb_x2l_merge true false)
          (Collision|SetCollisionEnabled _sm_road_citycurb_x2l_merge "QueryAndPhysics")
          (Variables|Default|SetIntersectionSelect 2)
          (goto _label)
          (elif (Variables|Default|GetIntersection%20SideWalk?)
            (Rendering|SetVisibility _sm_road_citycurbwalk_merge true false)
            (Collision|SetCollisionEnabled _sm_road_citycurbwalk_merge "QueryAndPhysics")
            (Variables|Default|SetIntersectionSelect 3)
            (goto _label)
            (elif (Variables|Default|GetIntersection%20SideWalkX2?)
              (Rendering|SetVisibility _sm_road_citycurbwalk_x2l_merge true false)
              (Collision|SetCollisionEnabled _sm_road_citycurbwalk_x2l_merge "QueryAndPhysics")
              (Variables|Default|SetIntersectionSelect 4)
              (goto _label)
              (elif (Variables|Default|GetIntersection%20Highway?)
                (Rendering|SetVisibility _sm_road_highway_merge true false)
                (Collision|SetCollisionEnabled _sm_road_highway_merge "QueryAndPhysics")
                (Variables|Default|SetIntersectionSelect 5)
                (goto _label)
                (elif (Variables|Default|GetIntersection%20HighwayX2?)
                  (Rendering|SetVisibility _sm_road_highway_x2l_merge true false)
                  (Collision|SetCollisionEnabled _sm_road_highway_x2l_merge "QueryAndPhysics")
                  (Variables|Default|SetIntersectionSelect 6)
                  (goto _label)
                  (elif (Variables|Default|GetIntersection%20SingleLane?)
                    (Rendering|SetVisibility _sm_road_singlelane_merge true false)
                    (Collision|SetCollisionEnabled _sm_road_singlelane_merge "QueryAndPhysics")
                    (Variables|Default|SetIntersectionSelect 7)
                    (goto _label)))))))))
    (:then_1
      ;[1 1 1] Sets correct Mesh socket Setup
      (Transformation|AttachComponentToComponent (Variables|Default|GetAttach%20Road%20Start) (Utilities|Array|Get(acopy) (Utilities|Array|MakeArray 0 (Variables|Default|GetSM_Road_CityCurb_Merge) (Variables|Default|GetSM_Road_CityCurb_X2L_Merge) (Variables|Default|GetSM_Road_CityCurbWalk_Merge) (Variables|Default|GetSM_Road_CityCurbWalk_X2L_Merge) (Variables|Default|GetSM_Road_Highway_Merge) (Variables|Default|GetSM_Road_Highway_X2L_Merge) (Variables|Default|GetSM_Road_SingleLane_Merge)) (Variables|Default|GetIntersectionSelect)) "SocketStart" "SnapToTarget" "SnapToTarget" "KeepWorld" false)
      (Transformation|AttachComponentToComponent (Variables|Default|GetAttach%20Road%20End) (Utilities|Array|Get(acopy) (Utilities|Array|MakeArray 0 (Variables|Default|GetSM_Road_CityCurb_Merge) (Variables|Default|GetSM_Road_CityCurb_X2L_Merge) (Variables|Default|GetSM_Road_CityCurbWalk_Merge) (Variables|Default|GetSM_Road_CityCurbWalk_X2L_Merge) (Variables|Default|GetSM_Road_Highway_Merge) (Variables|Default|GetSM_Road_Highway_X2L_Merge) (Variables|Default|GetSM_Road_SingleLane_Merge)) (Variables|Default|GetIntersectionSelect)) "SocketEnd" "SnapToTarget" "SnapToTarget" "KeepWorld" false)
      (Transformation|AttachComponentToComponent (Variables|Default|GetAttach%20Road%20Merge) (Utilities|Array|Get(acopy) (Utilities|Array|MakeArray 0 (Variables|Default|GetSM_Road_CityCurb_Merge) (Variables|Default|GetSM_Road_CityCurb_X2L_Merge) (Variables|Default|GetSM_Road_CityCurbWalk_Merge) (Variables|Default|GetSM_Road_CityCurbWalk_X2L_Merge) (Variables|Default|GetSM_Road_Highway_Merge) (Variables|Default|GetSM_Road_Highway_X2L_Merge) (Variables|Default|GetSM_Road_SingleLane_Merge)) (Variables|Default|GetIntersectionSelect)) "SocketMerge" "SnapToTarget" "SnapToTarget" "KeepWorld" false))))