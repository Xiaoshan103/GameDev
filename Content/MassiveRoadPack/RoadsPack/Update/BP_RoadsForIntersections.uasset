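; Road variant Blueprint that offers an easy selector for road meshes that work with the newer intersections and mergers.
; Its construction script calls the parent's script, then sets SelectSplineMesh1 from a prioritized chain of boolean toggles where the first true one wins.
; The toggles cover curb, sidewalk and highway roads, each with an X2 variant, plus single lane; with none set, the mesh stays unchanged.
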(event EventBeginPlay)

(event Collision|EventActorBeginOverlap
  (params (OtherActor :type Actor%20Object%20Reference)))

(event EventTick
  (params (DeltaSeconds :type Float%20%28single-precision%29)))

(fn ConstructionScript
  (|CallParentFunction)
  (Utilities|FlowControl|Sequence
    (:then_0
      ;[1 1 1] Ease Selector for New Roads that work with new Intersections and Mergers
      (if (Variables|EAZYSELECTOR(DoubleClicktoSelect)|GetRoad%20Curb?)
        (Variables|Default|SetSelect%20SplineMesh1 "/Game/MassiveRoadPack/RoadsPack/Meshes/Intersections/SM_Road_CityCurb.SM_Road_CityCurb")
        (elif (Variables|EAZYSELECTOR(DoubleClicktoSelect)|GetRoad%20CurbX2?)
          (Variables|Default|SetSelect%20SplineMesh1 "/Game/MassiveRoadPack/RoadsPack/Meshes/Intersections/SM_Road_CityCurb_X2L.SM_Road_CityCurb_X2L")
          (elif (Variables|EAZYSELECTOR(DoubleClicktoSelect)|GetRoad%20SideWalk?)
            (Variables|Default|SetSelect%20SplineMesh1 "/Game/MassiveRoadPack/RoadsPack/Meshes/Intersections/SM_Road_CityCurbWalk.SM_Road_CityCurbWalk")
            (elif (Variables|EAZYSELECTOR(DoubleClicktoSelect)|GetRoad%20SideWalkX2?)
              (Variables|Default|SetSelect%20SplineMesh1 "/Game/MassiveRoadPack/RoadsPack/Meshes/Intersections/SM_Road_CityCurbWalk_X2L.SM_Road_CityCurbWalk_X2L")
              (elif (Variables|EAZYSELECTOR(DoubleClicktoSelect)|GetRoad%20Highway?)
                (Variables|Default|SetSelect%20SplineMesh1 "/Game/MassiveRoadPack/RoadsPack/Meshes/Intersections/SM_Road_Highway.SM_Road_Highway")
                (elif (Variables|EAZYSELECTOR(DoubleClicktoSelect)|GetRoad%20HighwayX2?)
                  (Variables|Default|SetSelect%20SplineMesh1 "/Game/MassiveRoadPack/RoadsPack/Meshes/Intersections/SM_Road_Highway_X2L.SM_Road_Highway_X2L")
                  (elif (Variables|EAZYSELECTOR(DoubleClicktoSelect)|GetRoad%20SingleLane?)
                    (Variables|Default|SetSelect%20SplineMesh1 "/Game/MassiveRoadPack/RoadsPack/Meshes/Intersections/SM_Road_SingleLane.SM_Road_SingleLane")))))))))))