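; Road intersection Blueprint that offers eleven four-way and three-way mesh variants: curb, sidewalk, highway and single-lane styles.
; Its construction script checks boolean options in priority order, then makes the first match visible, enables its collision and records its index in IntersectionSelect.
; That index picks the parent mesh whose X and Y sockets the AttachRoad components snap to, keeping world scale.
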(fn ConstructionScript
  (bind _sm_road_singlelane_int (Variables|Default|GetSM_Road_SingleLane_INT))
  (bind _sm_road_highway_int (Variables|Default|GetSM_Road_Highway_INT))
  (bind _sm_road_highway_x2l_int (Variables|Default|GetSM_Road_Highway_X2L_INT))
  (bind _sm_road_citycurb_3way (Variables|Default|GetSM_Road_CityCurb_3Way))
  (bind _sm_road_citycurb_x2l_3way (Variables|Default|GetSM_Road_CityCurb_X2L_3Way))
  (bind _sm_road_citycurbwalk_3way (Variables|Default|GetSM_Road_CityCurbWalk_3Way))
  (bind _sm_road_citycurb_int (Variables|Default|GetSM_Road_CityCurb_INT))
  (bind _sm_road_citycurb_x2l_int (Variables|Default|GetSM_Road_CityCurb_X2L_INT))
  (bind _sm_road_citycurbwalk_int (Variables|Default|GetSM_Road_CityCurbWalk_INT))
  (bind _sm_road_citycurbwalk_x2l_int (Variables|Default|GetSM_Road_CityCurbWalk_X2L_INT))
  (bind _sm_road_citycurbwalk_x2l_3way (Variables|Default|GetSM_Road_CityCurbWalk_X2L_3Way))
  (Utilities|FlowControl|Sequence
    (:then_0
      ;[1 1 1] selection process
      (if (Variables|Default|GetIntersection%20Curb?)
        (Rendering|SetVisibility _sm_road_citycurb_int true false)
        (Collision|SetCollisionEnabled _sm_road_citycurb_int "QueryAndPhysics")
        (Variables|Default|SetIntersectionSelect 0)
        (elif (Variables|Default|GetIntersection%20CurbX2?)
          (Rendering|SetVisibility _sm_road_citycurb_x2l_int true false)
          (Collision|SetCollisionEnabled _sm_road_citycurb_x2l_int "QueryAndPhysics")
          (Variables|Default|SetIntersectionSelect 1)
          (elif (Variables|Default|GetIntersection%20SideWalk?)
            (Rendering|SetVisibility _sm_road_citycurbwalk_int true false)
            (Collision|SetCollisionEnabled _sm_road_citycurbwalk_int "QueryAndPhysics")
            (Variables|Default|SetIntersectionSelect 2)
            (elif (Variables|Default|GetIntersection%20SideWalkX2?)
              (Rendering|SetVisibility _sm_road_citycurbwalk_x2l_int true false)
              (Collision|SetCollisionEnabled _sm_road_citycurbwalk_x2l_int "QueryAndPhysics")
              (Variables|Default|SetIntersectionSelect 3)
              (elif (Variables|Default|GetIntersection%20Highway?)
                (Rendering|SetVisibility _sm_road_highway_int true false)
                (Collision|SetCollisionEnabled _sm_road_highway_int "QueryAndPhysics")
                (Variables|Default|SetIntersectionSelect 4)
                (elif (Variables|Default|GetIntersection%20HighwayX2?)
                  (Rendering|SetVisibility _sm_road_highway_x2l_int true false)
                  (Collision|SetCollisionEnabled _sm_road_highway_x2l_int "QueryAndPhysics")
                  (Variables|Default|SetIntersectionSelect 5)
                  (elif (Variables|Default|GetIntersection%20SingleLane?)
                    (Rendering|SetVisibility _sm_road_singlelane_int true false)
                    (Collision|SetCollisionEnabled _sm_road_singlelane_int "QueryAndPhysics")
                    (Variables|Default|SetIntersectionSelect 6)
                    (elif (Variables|Default|Get3Way_Curb?)
                      (Rendering|SetVisibility _sm_road_citycurb_3way true false)
                      (Collision|SetCollisionEnabled _sm_road_citycurb_3way "QueryAndPhysics")
                      (Variables|Default|SetIntersectionSelect 7)
                      (elif (Variables|Default|Get3Way_CurbX2?)
                        (Rendering|SetVisibility _sm_road_citycurb_x2l_3way true false)
                        (Collision|SetCollisionEnabled _sm_road_citycurb_x2l_3way "QueryAndPhysics")
                        (Variables|Default|SetIntersectionSelect 8)
                        (elif (Variables|Default|Get3Way_SideWalk?)
                          (Rendering|SetVisibility _sm_road_citycurbwalk_3way true false)
                          (Collision|SetCollisionEnabled _sm_road_citycurbwalk_3way "QueryAndPhysics")
                          (Variables|Default|SetIntersectionSelect 9)
                          (elif (Variables|Default|Get3Way_SideWalkX2?)
                            (Rendering|SetVisibility _sm_road_citycurbwalk_x2l_3way true false)
                            (Collision|SetCollisionEnabled _sm_road_citycurbwalk_x2l_3way "QueryAndPhysics")
                            (Variables|Default|SetIntersectionSelect 10)))))))))))))
    (:then_1
      ;[1 1 1] Sets correct Mesh socket Setup
      (Transformation|AttachComponentToComponent (Variables|Default|GetAttach%20Road%20X+) (Utilities|Array|Get(acopy) (Utilities|Array|MakeArray (Variables|Default|GetSM_Road_CityCurb_INT) (Variables|Default|GetSM_Road_CityCurb_X2L_INT) (Variables|Default|GetSM_Road_CityCurbWalk_INT) (Variables|Default|GetSM_Road_CityCurbWalk_X2L_INT) (Variables|Default|GetSM_Road_Highway_INT) (Variables|Default|GetSM_Road_Highway_X2L_INT) (Variables|Default|GetSM_Road_SingleLane_INT) (Variables|Default|GetSM_Road_CityCurb_3Way) (Variables|Default|GetSM_Road_CityCurb_X2L_3Way) (Variables|Default|GetSM_Road_CityCurbWalk_3Way) (Variables|Default|GetSM_Road_CityCurbWalk_X2L_3Way)) (Variables|Default|GetIntersectionSelect)) "SocketX+" "SnapToTarget" "SnapToTarget" "KeepWorld" true)
      (Transformation|AttachComponentToComponent (Variables|Default|GetAttach%20Road%20X-) (Utilities|Array|Get(acopy) (Utilities|Array|MakeArray (Variables|Default|GetSM_Road_CityCurb_INT) (Variables|Default|GetSM_Road_CityCurb_X2L_INT) (Variables|Default|GetSM_Road_CityCurbWalk_INT) (Variables|Default|GetSM_Road_CityCurbWalk_X2L_INT) (Variables|Default|GetSM_Road_Highway_INT) (Variables|Default|GetSM_Road_Highway_X2L_INT) (Variables|Default|GetSM_Road_SingleLane_INT) (Variables|Default|GetSM_Road_CityCurb_3Way) (Variables|Default|GetSM_Road_CityCurb_X2L_3Way) (Variables|Default|GetSM_Road_CityCurbWalk_3Way) (Variables|Default|GetSM_Road_CityCurbWalk_X2L_3Way)) (Variables|Default|GetIntersectionSelect)) "SocketX-" "SnapToTarget" "SnapToTarget" "KeepWorld" true)
      (Transformation|AttachComponentToComponent (Variables|Default|GetAttach%20Road%20Y+) (Utilities|Array|Get(acopy) (Utilities|Array|MakeArray (Variables|Default|GetSM_Road_CityCurb_INT) (Variables|Default|GetSM_Road_CityCurb_X2L_INT) (Variables|Default|GetSM_Road_CityCurbWalk_INT) (Variables|Default|GetSM_Road_CityCurbWalk_X2L_INT) (Variables|Default|GetSM_Road_Highway_INT) (Variables|Default|GetSM_Road_Highway_X2L_INT) (Variables|Default|GetSM_Road_SingleLane_INT) (Variables|Default|GetSM_Road_CityCurb_3Way) (Variables|Default|GetSM_Road_CityCurb_X2L_3Way) (Variables|Default|GetSM_Road_CityCurbWalk_3Way) (Variables|Default|GetSM_Road_CityCurbWalk_X2L_3Way)) (Variables|Default|GetIntersectionSelect)) "SocketY+" "SnapToTarget" "SnapToTarget" "KeepWorld" true)
      (Transformation|AttachComponentToComponent (Variables|Default|GetAttach%20Road%20Y-) (Utilities|Array|Get(acopy) (Utilities|Array|MakeArray (Variables|Default|GetSM_Road_CityCurb_INT) (Variables|Default|GetSM_Road_CityCurb_X2L_INT) (Variables|Default|GetSM_Road_CityCurbWalk_INT) (Variables|Default|GetSM_Road_CityCurbWalk_X2L_INT) (Variables|Default|GetSM_Road_Highway_INT) (Variables|Default|GetSM_Road_Highway_X2L_INT) (Variables|Default|GetSM_Road_SingleLane_INT) (Variables|Default|GetSM_Road_CityCurb_3Way) (Variables|Default|GetSM_Road_CityCurb_X2L_3Way) (Variables|Default|GetSM_Road_CityCurbWalk_3Way) (Variables|Default|GetSM_Road_CityCurbWalk_X2L_3Way)) (Variables|Default|GetIntersectionSelect)) "SocketY-" "SnapToTarget" "SnapToTarget" "KeepWorld" true))))