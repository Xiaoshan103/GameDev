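; BP_Road is a spline-based road actor that builds its geometry in the Construction Script; its runtime events are empty.
; Three optional spline mesh layers deform along the spline at set spacings, and three static mesh layers place props with seeded random yaw or a local offset.
; The first layer also moves TraceObject to the spline's end and snaps an optional AttachEndActor to it.
; A basic mode instead spans one spline mesh per point pair.
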(event EventBeginPlay)

(event Collision|EventActorBeginOverlap
  (params (OtherActor :type Actor%20Object%20Reference)))

(event EventTick
  (params (DeltaSeconds :type Float%20%28single-precision%29)))

(fn ConstructionScript
  (bind _spline (Variables|Default|GetSpline))
  (bind _splinemesh1_spacing (Variables|Spline1|GetSplineMesh1%20Spacing))
  (bind _splinemesh1_tangent_scale (Variables|Spline1|GetSplineMesh1%20Tangent%20Scale))
  (bind _spline_2 (Variables|Default|GetSpline))
  (bind _spline_3 (Variables|Default|GetSpline))
  (bind _splinemesh1_offset (Variables|Spline1|GetSplineMesh1%20Offset))
  (bind _splinemesh2_offset (Variables|Spline2|GetSplineMesh2%20Offset))
  (bind _splinemesh3_offset (Variables|Spline3|GetSplineMesh3%20Offset))
  (bind _splinemesh3_spacing (Variables|Spline3|GetSplineMesh3%20Spacing))
  (bind _spline_4 (Variables|Default|GetSpline))
  (bind _splinemesh3_spacing_2 (Variables|Spline3|GetSplineMesh3%20Spacing))
  (bind _splinemesh2_spacing (Variables|Spline2|GetSplineMesh2%20Spacing))
  (bind _splinemesh2_spacing_2 (Variables|Spline2|GetSplineMesh2%20Spacing))
  (bind _staticmesh2_collison (Variables|Mesh2|GetStaticMesh2%20Collison))
  (bind _attachendactor (Variables|EAZYSELECTOR(DoubleClicktoSelect)|GetAttachEndActor))
  (bind _spline_5 (Variables|Default|GetSpline))
  (bind _staticmeshes_spacing3 (Variables|Mesh3|GetStaticMeshes%20Spacing3))
  (bind _select_staticmeshes3 (Variables|Mesh3|GetSelect%20StaticMeshes3))
  (bind _spline_6 (Variables|Default|GetSpline))
  (bind _selectstatic3_meshesmaterial (Variables|Mesh3|GetSelectStatic3%20MeshesMaterial))
  (bind _traceobject (Variables|Default|GetTraceObject))
  (bind _staticmesh3_collison (Variables|Mesh3|GetStaticMesh3%20Collison))
  (bind _spline_7 (Variables|Default|GetSpline))
  (bind _spline_8 (Variables|Default|GetSpline))
  (bind _staticmeshes_spacing2 (Variables|Mesh2|GetStaticMeshes%20Spacing2))
  (bind _staticmeshes_spacing (Variables|Mesh1|GetStaticMeshes%20Spacing))
  (bind _select_staticmeshes (Variables|Mesh1|GetSelect%20StaticMeshes))
  (bind _selectstaticmeshesmaterial (Variables|Mesh1|GetSelectStaticMeshesMaterial))
  (bind _staticmesh_collison (Variables|Mesh1|GetStaticMesh%20Collison))
  (bind _select_staticmeshes2 (Variables|Mesh2|GetSelect%20StaticMeshes2))
  (bind _selectstatic2_meshesmaterial (Variables|Mesh2|GetSelectStatic2%20MeshesMaterial))
  (bind _returnvalue (Spline|GetNumberOfSplinePoints _spline_7))
  (bind _returnvalue_2 (Spline|GetTransformatSplinePoint _spline_7 _returnvalue "World" false))
  (Utilities|FlowControl|Sequence
    (:then_0
      (Utilities|FlowControl|Sequence
        (:then_0
          (Utilities|FlowControl|Sequence
            (:then_0
              ;[1 0.43 0.43] Add SplineMesh (will deform to spline)
              (if (Variables|Spline1|GetAdd%20SplineMesh1?)
                (for _index (range 0 (.ReturnValue (Math|Float|Division(WholeandRemainder) (Spline|GetSplineLength _spline_3) _splinemesh1_spacing)))
                  (bind _output_get (Variables|Default|SetIndexLoop _index))
                  (bind _returnvalue_3 (AddComponent|AddSplineMeshComponent true))
                  (bind _output_get_2 (Variables|Default|SetLocalSplineMesh1 _returnvalue_3))
                  (Components|StaticMesh|SetStaticMesh _output_get_2 (Variables|Spline1|GetSelect%20SplineMesh1))
                  (Rendering|Material|SetMaterial _output_get_2 0 (Variables|Spline1|GetSelect%20SplineMesh1%20Material))
                  (SplineMesh|SetForwardAxis _output_get_2 (Variables|Spline1|GetSplineMesh1%20ForwardAxis) true)
                  (Rendering|SetCastShadow _output_get_2 (Variables|Spline1|GetSplineMesh1%20CastShadows?))
                  (SplineMesh|SetStartandEnd _output_get_2 (+ (Spline|GetLocationatDistanceAlongSpline _spline_3 (* _output_get _splinemesh1_spacing) "World") (Math|Vector|MakeVector 0.0 0.0 _splinemesh1_offset)) (* (Spline|GetDirectionatDistanceAlongSpline _spline_3 (* _output_get _splinemesh1_spacing) "World") _splinemesh1_tangent_scale) (+ (Spline|GetLocationatDistanceAlongSpline _spline_3 (+ (* _output_get _splinemesh1_spacing) _splinemesh1_spacing) "World") (Math|Vector|MakeVector 0.0 0.0 _splinemesh1_offset)) (* (Spline|GetDirectionatDistanceAlongSpline _spline_3 (+ (* _output_get _splinemesh1_spacing) _splinemesh1_spacing) "World") _splinemesh1_tangent_scale) true :!class /Script/Engine.SplineMeshComponent)
                  (Collision|SetCollisionEnabled _output_get_2 (Variables|Spline1|GetSplineMesh1%20Collison))
                  (Transformation|SetWorldRotation _traceobject (.rotation _returnvalue_2) false false)
                  (Transformation|SetWorldLocation _traceobject (.location _returnvalue_2) false false)
                  (Utilities|IsValid _attachendactor
                    (:Is%20Valid
                      (Transformation|AttachComponentToComponent _attachendactor _traceobject "None" "SnapToTarget" "SnapToTarget" "KeepWorld" false))))))
            (:then_1
              ;[1 0.43 0.43] Add SplineMesh2 (will deform to spline)
              (if (Variables|Spline2|GetAdd%20SplineMesh2?)
                (for _index_2 (range 0 (.ReturnValue (Math|Float|Division(WholeandRemainder) (Spline|GetSplineLength _spline_4) _splinemesh2_spacing)))
                  (bind _returnvalue_4 (AddComponent|AddSplineMeshComponent true))
                  (bind _output_get_3 (Variables|Default|SetLocalSplineMesh2 _returnvalue_4))
                  (Components|StaticMesh|SetStaticMesh _output_get_3 (Variables|Spline2|GetSelect%20SplineMesh2))
                  (Rendering|Material|SetMaterial _output_get_3 0 (Variables|Spline2|GetSelect%20SplineMesh2%20Material))
                  (SplineMesh|SetForwardAxis _output_get_3 (Variables|Spline2|GetSplineMesh2%20ForwardAxis) true)
                  (Rendering|SetCastShadow _output_get_3 (Variables|Spline2|GetSplineMesh2%20CastShadows?))
                  (SplineMesh|SetStartandEnd _output_get_3 (+ (Spline|GetLocationatDistanceAlongSpline _spline_4 (* _index_2 _splinemesh2_spacing) "World") (Math|Vector|MakeVector 0.0 0.0 _splinemesh2_offset)) (* (Spline|GetDirectionatDistanceAlongSpline _spline_4 (* _index_2 _splinemesh2_spacing) "World") _splinemesh2_spacing_2) (+ (Spline|GetLocationatDistanceAlongSpline _spline_4 (+ (* _index_2 _splinemesh2_spacing) _splinemesh2_spacing) "World") (Math|Vector|MakeVector 0.0 0.0 _splinemesh2_offset)) (* (Spline|GetDirectionatDistanceAlongSpline _spline_4 (+ (* _index_2 _splinemesh2_spacing) _splinemesh2_spacing) "World") _splinemesh2_spacing_2) true :!class /Script/Engine.SplineMeshComponent)
                  (Collision|SetCollisionEnabled _output_get_3 (Variables|Spline2|GetSplineMesh2%20Collison)))))
            (:then_2
              ;[1 0.43 0.43] Add SplineMesh2 (will deform to spline)
              (if (Variables|Spline3|GetAdd%20SplineMesh3?)
                (for _index_3 (range 0 (.ReturnValue (Math|Float|Division(WholeandRemainder) (Spline|GetSplineLength _spline_2) _splinemesh3_spacing)))
                  (bind _returnvalue_5 (AddComponent|AddSplineMeshComponent true))
                  (bind _output_get_4 (Variables|Default|SetLocalSplineMesh3 _returnvalue_5))
                  (Components|StaticMesh|SetStaticMesh _output_get_4 (Variables|Spline3|GetSelect%20SplineMesh3))
                  (Rendering|Material|SetMaterial _output_get_4 0 (Variables|Spline3|GetSelect%20SplineMesh3%20Material))
                  (SplineMesh|SetForwardAxis _output_get_4 (Variables|Spline3|GetSplineMesh3%20ForwardAxis) true)
                  (Rendering|SetCastShadow _output_get_4 (Variables|Spline3|GetSplineMesh3%20CastShadows?))
                  (SplineMesh|SetStartandEnd _output_get_4 (+ (Spline|GetLocationatDistanceAlongSpline _spline_2 (* _index_3 _splinemesh3_spacing) "World") (Math|Vector|MakeVector 0.0 0.0 _splinemesh3_offset)) (* (Spline|GetDirectionatDistanceAlongSpline _spline_2 (* _index_3 _splinemesh3_spacing) "World") _splinemesh3_spacing_2) (+ (Spline|GetLocationatDistanceAlongSpline _spline_2 (+ (* _index_3 _splinemesh3_spacing) _splinemesh3_spacing) "World") (Math|Vector|MakeVector 0.0 0.0 _splinemesh3_offset)) (* (Spline|GetDirectionatDistanceAlongSpline _spline_2 (+ (* _index_3 _splinemesh3_spacing) _splinemesh3_spacing) "World") _splinemesh3_spacing_2) true :!class /Script/Engine.SplineMeshComponent)
                  (Collision|SetCollisionEnabled _output_get_4 (Variables|Spline3|GetSplineMesh3%20Collison)))))))
        (:then_1
          ;[0.4799 0.5036 1] Add Static Meshes Along Spline (With optional Random Rotation)
          (if (Variables|Mesh1|GetAdd%20StaticMeshes%20Along%20Spline?)
            (for _index_4 (range 0 (.ReturnValue (Math|Float|Division(WholeandRemainder) (Spline|GetSplineLength _spline_8) _staticmeshes_spacing)))
              (if (Variables|Mesh1|GetStaticMeshes%20RandomRotate?)
                ;;[1 1 1] RandomRotator Object Along Spline
                (bind _returnvalue_6 (AddComponent|AddStaticMeshComponent true (Math|Transform|MakeTransform (Spline|GetLocationatDistanceAlongSpline _spline_8 (* _index_4 _staticmeshes_spacing) "World") (Math|Rotator|CombineRotators (Spline|GetRotationatDistanceAlongSpline _spline_8 (* _index_4 _staticmeshes_spacing) "World") (Math|Rotator|MakeRotator 0.0 0.0 (Math|Random|RandomFloatinRangefromStream 0.0 3.6e+02 (Variables|Mesh1|GetRandomStream)))))))
                (Components|StaticMesh|SetStaticMesh _returnvalue_6 _select_staticmeshes)
                (Rendering|Material|SetMaterial _returnvalue_6 0 _selectstaticmeshesmaterial)
                (Collision|SetCollisionEnabled _returnvalue_6 _staticmesh_collison)
                (else
                  (bind _returnvalue_7 (AddComponent|AddStaticMeshComponent true (Math|Transform|MakeTransform (Spline|GetLocationatDistanceAlongSpline _spline_8 (* _index_4 _staticmeshes_spacing) "World") (Spline|GetRotationatDistanceAlongSpline _spline_8 (* _index_4 _staticmeshes_spacing) "World"))))
                  (bind _output_get_5 (Variables|Mesh1|SetStaticSplineMesh1 _returnvalue_7))
                  (Transformation|AddLocalOffset _output_get_5 (Variables|Mesh1|GetStaticMesh%201%20LocalOffset) false false)
                  (Components|StaticMesh|SetStaticMesh _output_get_5 _select_staticmeshes)
                  (Rendering|Material|SetMaterial _returnvalue_7 0 _selectstaticmeshesmaterial)
                  (Collision|SetCollisionEnabled _returnvalue_7 _staticmesh_collison))))))
        (:then_2
          ;[0.4799 0.5036 1] Add Static Meshes Along Spline (With optional Random Rotation)
          (if (Variables|Mesh2|GetAdd%20StaticMeshes2%20Along%20Spline?)
            (for _index_5 (range 0 (.ReturnValue (Math|Float|Division(WholeandRemainder) (Spline|GetSplineLength _spline_6) _staticmeshes_spacing2)))
              (if (Variables|Mesh2|GetStaticMeshes2%20RandomRotate?)
                ;;[1 1 1] RandomRotator Object Along Spline
                (bind _returnvalue_8 (AddComponent|AddStaticMeshComponent true (Math|Transform|MakeTransform (Spline|GetLocationatDistanceAlongSpline _spline_6 (* _index_5 _staticmeshes_spacing2) "World") (Math|Rotator|CombineRotators (Spline|GetRotationatDistanceAlongSpline _spline_6 (* _index_5 _staticmeshes_spacing2) "World") (Math|Rotator|MakeRotator 0.0 0.0 (Math|Random|RandomFloatinRangefromStream 0.0 3.6e+02 (Variables|Mesh1|GetRandomStream)))))))
                (Components|StaticMesh|SetStaticMesh _returnvalue_8 _select_staticmeshes2)
                (Rendering|Material|SetMaterial _returnvalue_8 0 _selectstatic2_meshesmaterial)
                (Collision|SetCollisionEnabled _returnvalue_8 _staticmesh2_collison)
                (else
                  (bind _returnvalue_9 (AddComponent|AddStaticMeshComponent true (Math|Transform|MakeTransform (Spline|GetLocationatDistanceAlongSpline _spline_6 (* _index_5 _staticmeshes_spacing2) "World") (Spline|GetRotationatDistanceAlongSpline _spline_6 (* _index_5 _staticmeshes_spacing2) "World"))))
                  (bind _output_get_6 (Variables|Mesh2|SetStaticSplineMesh2 _returnvalue_9))
                  (Transformation|AddLocalOffset _output_get_6 (Variables|Mesh2|GetStaticMesh2%20LocalOffset) false false)
                  (Components|StaticMesh|SetStaticMesh _output_get_6 _select_staticmeshes2)
                  (Rendering|Material|SetMaterial _returnvalue_9 0 _selectstatic2_meshesmaterial)
                  (Collision|SetCollisionEnabled _returnvalue_9 _staticmesh2_collison))))))
        (:then_3
          ;[0.4799 0.5036 1] Add Static Meshes Along Spline (With optional Random Rotation)
          (if (Variables|Mesh3|GetAdd%20StaticMeshes3%20Along%20Spline?)
            (for _index_6 (range 0 (.ReturnValue (Math|Float|Division(WholeandRemainder) (Spline|GetSplineLength _spline_5) _staticmeshes_spacing3)))
              (if (Variables|Mesh3|GetStaticMeshes3%20RandomRotate?)
                ;;[1 1 1] RandomRotator Object Along Spline
                (bind _returnvalue_10 (AddComponent|AddStaticMeshComponent true (Math|Transform|MakeTransform (Spline|GetLocationatDistanceAlongSpline _spline_5 (* _index_6 _staticmeshes_spacing3) "World") (Math|Rotator|CombineRotators (Spline|GetRotationatDistanceAlongSpline _spline_5 (* _index_6 _staticmeshes_spacing3) "World") (Math|Rotator|MakeRotator 0.0 0.0 (Math|Random|RandomFloatinRangefromStream 0.0 3.6e+02 (Variables|Mesh3|GetRandomStream3)))))))
                (Components|StaticMesh|SetStaticMesh _returnvalue_10 _select_staticmeshes3)
                (Rendering|Material|SetMaterial _returnvalue_10 0 _selectstatic3_meshesmaterial)
                (Collision|SetCollisionEnabled _returnvalue_10 _staticmesh3_collison)
                (else
                  (bind _returnvalue_11 (AddComponent|AddStaticMeshComponent true (Math|Transform|MakeTransform (Spline|GetLocationatDistanceAlongSpline _spline_5 (* _index_6 _staticmeshes_spacing3) "World") (Spline|GetRotationatDistanceAlongSpline _spline_5 (* _index_6 _staticmeshes_spacing3) "World"))))
                  (bind _output_get_7 (Variables|Mesh1|SetStaticSplineMesh1 _returnvalue_11))
                  (Transformation|AddLocalOffset _output_get_7 (Variables|Mesh3|GetStaticMesh3%20LocalOffset) false false)
                  (Components|StaticMesh|SetStaticMesh _output_get_7 _select_staticmeshes3)
                  (Rendering|Material|SetMaterial _returnvalue_11 0 _selectstatic3_meshesmaterial)
                  (Collision|SetCollisionEnabled _returnvalue_11 _staticmesh3_collison))))))))
    (:then_1
      ;[1 1 1] Causes construction Script to reactive inorder to update splines without modifing setup
      (if (Variables|EAZYSELECTOR(DoubleClicktoSelect)|GetUPDATE%20SPLINES?)
        _))
    (:then_2
      ;[1 1 1] BasicSplineFunctionality
      (if (Variables|BasicSpline|GetBasic%20Spline?)
        (for _index_7 (range 0 (- (Spline|GetNumberOfSplinePoints _spline) 2))
          ;;[1 0.25 0.25] Replace your Spline Mesh Here
          (bind _returnvalue_12 (AddComponent|AddSplineMeshComponent true))
          (bind _output_get_8 (Variables|Default|SetBasicSpline _returnvalue_12))
          (Rendering|Material|SetMaterial _output_get_8 0 (Variables|BasicSpline|GetSelect%20Basic%20Spline%20Material))
          (Transformation|AttachComponentToComponent _output_get_8 0 "None" "KeepRelative" "KeepRelative" "KeepRelative" true)
          (SplineMesh|SetForwardAxis _output_get_8 (Variables|BasicSpline|GetBasic%20Spline%20ForwardAxis) true)
          (SplineMesh|SetStartandEnd _output_get_8 (.Location (Spline|GetLocationandTangentatSplinePoint _spline _index_7 "World")) (.Tangent (Spline|GetLocationandTangentatSplinePoint _spline _index_7 "World")) (.Location (Spline|GetLocationandTangentatSplinePoint _spline (+ _index_7 1) "World")) (.Tangent (Spline|GetLocationandTangentatSplinePoint _spline (+ _index_7 1) "World")) true :!class /Script/Engine.SplineMeshComponent)
          (Collision|SetCollisionEnabled _returnvalue_12 (Variables|BasicSpline|GetBasic%20Spline%20Collison)))))))